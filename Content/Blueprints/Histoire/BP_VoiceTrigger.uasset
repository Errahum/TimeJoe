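; BP_VoiceTrigger is a trigger actor that plays a configurable voice line through the player's BP_FirstPersonCharacter after a delay.
; Any actor overlap starts the delay, guarded by a DoOnce so the line is triggered once.
; With MustStayIn set, it checks after the delay that a BP_FirstPersonCharacter still overlaps, and otherwise resets the DoOnce so a later overlap can retry.
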(event Custom|Event%20ResetVoiceLine
  (Utilities|FlowControl|DoOnce false) ; enters at Reset
)

(event EventBeginPlay)

(event Collision|EventActorBeginOverlap
  (params (OtherActor :type Actor%20Object%20Reference))
  (Utilities|FlowControl|DoOnce false
    (:Completed
      (Development|PrintString "Voice line Delay Start" true true "(R=0.000000,G=1.000000,B=0.335798,A=1.000000)")
      (Utilities|FlowControl|Delay (Variables|Default|GetDelay))
      (if (Variables|Default|GetMustStayIn)
        (if (Utilities|Array|IsEmpty (Collision|GetOverlappingActors "/Game/FirstPerson/Blueprints/BP_FirstPersonCharacter.BP_FirstPersonCharacter_C" :!class /Script/Engine.Actor))
          (CallFunction|EventResetVoiceLine)
          (else
            (bind _asbp_first_person_character (Utilities|Casting|CastToBP_FirstPersonCharacter (Game|GetPlayerCharacter 0) :!label _label))
            (Default|PlayVoiceLine _asbp_first_person_character (Variables|Default|GetVoiceLine))))
        (else
          (goto _label))))))

(event EventTick
  (params (DeltaSeconds :type Float%20%28single-precision%29)))

(fn ConstructionScript)