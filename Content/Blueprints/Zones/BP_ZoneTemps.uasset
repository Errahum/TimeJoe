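; Base actor for time zones, with Fast, Slow and Stop children, that affect overlapping actors tagged Player, Physic or Timeline.
; On begin play and tagged overlap, it loops overlapping actors, stores each actor and tag, then calls AddEffect, empty here.
; On exit, it restores per-tag defaults for movement, damping or time dilation.
; It then re-runs UpdateMain on zones the actor still overlaps, so their effects reapply.
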(event OnComponentEndOverlap(Collision)
  (params (OverlappedComponent :type Primitive%20Component%20Object%20Reference) (OtherActor :type Actor%20Object%20Reference) (OtherComp :type Primitive%20Component%20Object%20Reference) (OtherBodyIndex :type Integer))
  ;[1 1 1] Lorsqu'on quitte la zone
  (bind _output_get (Variables|Default|SetOther%20Actor_End OtherActor))
  (bind _hastag (CallFunction|CheckObjectTag _output_get))
  (if _hastag
    (CallFunction|ResetEffect _output_get)
    (for (_ _array_index) (Collision|GetOverlappingActors _output_get "BP_ZoneTemps_C" :!class /Script/Engine.Actor)
      (bind _output_get_2 (Variables|Default|SetZoneUpdate (Utilities|Array|Get(acopy) (Collision|GetOverlappingActors _output_get "BP_ZoneTemps_C" :!class /Script/Engine.Actor) _array_index)))
      ;;[1 1 1] Update Fast
      (if (Actor|ActorHasTag _output_get_2 "Fast")
        (bind _asbp_zone_temps_fast (Utilities|Casting|CastToBP_ZoneTemps_Fast (Variables|Default|GetZoneUpdate))
          (:then
            (CallFunction|UpdateMain _asbp_zone_temps_fast)
            (Development|PrintString "Fast update" true true "(R=1.000000,G=0.811523,B=0.000000,A=1.000000)"))
          (:CastFailed
            (Development|PrintString "Fast Cast failed" true true "(R=1.000000,G=0.000000,B=0.017282,A=1.000000)")))
        (else
          ;;[1 1 1] Update Slow
          (if (Actor|ActorHasTag (Variables|Default|GetZoneUpdate) "Slow")
            (bind _asbp_zone_temps_slow (Utilities|Casting|CastToBP_ZoneTemps_Slow (Variables|Default|GetZoneUpdate))
              (:then
                (CallFunction|UpdateMain _asbp_zone_temps_slow)
                (Development|PrintString "Slow update" true true "(R=0.000000,G=0.033949,B=1.000000,A=1.000000)"))
              (:CastFailed
                (Development|PrintString "Slow Cast failed" true true "(R=1.000000,G=0.000000,B=0.017282,A=1.000000)")))
            (else
              ;;[1 1 1] Update Stop
              (if (Actor|ActorHasTag (Variables|Default|GetZoneUpdate) "Stop")
                (bind _asbp_zone_temps_stop (Utilities|Casting|CastToBP_ZoneTemps_Stop (Variables|Default|GetZoneUpdate))
                  (:then
                    (CallFunction|UpdateMain _asbp_zone_temps_stop)
                    (Development|PrintString "Stop update" true true "(R=0.300000,G=0.300000,B=0.300000,A=1.000000)"))
                  (:CastFailed
                    (Development|PrintString "Stop Cast failed" true true "(R=1.000000,G=0.000000,B=0.017282,A=1.000000)")))))))))))

(event OnComponentBeginOverlap(Collision)
  (params (OverlappedComponent :type Primitive%20Component%20Object%20Reference) (OtherActor :type Actor%20Object%20Reference) (OtherComp :type Primitive%20Component%20Object%20Reference) (OtherBodyIndex :type Integer) (bFromSweep :type Boolean) (SweepResult :type Hit%20Result%20Structure%20%28by%20ref%29))
  ;[1 1 1] À la création de la zone et à chaque fois qu'un object y entre, regarder chaque object pour voir ceux qui possèdent un Tag voulu. Retourne en string ce Tag, qui peut ensuite être accéder par les BP child des 3 zones pour déterminer comment l'object sera affecté par celles-ci
  (bind _hastag (CallFunction|CheckObjectTag OtherActor))
  (if _hastag
    (CallFunction|UpdateMain)))

(event Custom|ResetEffect
  (params (Other%20Actor :type Actor%20Object%20Reference))
  (bind _returnvalue (Game|GetPlayerCharacter 0))
  (bind _charactermovement (Variables|/Script/Engine.Character|GetCharacterMovement _returnvalue))
  ;[1 1 1] Lorsqu'un object sort d'une zone, rétablir ses propriétés par défaut selon le type d'objet (son Tag)
  ;;[1 1 1] Reset
  (bind _output_get (Variables|Default|SetResetActor Other%20Actor))
  (bind _tag (CallFunction|CheckObjectTag _output_get))
  (switch string _tag
    (:Player
      ;;[1 1 1] Reset Player
      (Variables|/Script/Engine.CharacterMovementComponent|SetJumpZVelocity _charactermovement 4.2e+02)
      (Variables|/Script/Engine.CharacterMovementComponent|SetMaxWalkSpeed _charactermovement 6e+02)
      (Variables|/Script/Engine.Actor|SetCustomTimeDilation _returnvalue 1.0)
      (Variables|/Script/Engine.CharacterMovementComponent|SetGravityScale _charactermovement 1.0)
      (Variables|/Script/Engine.CharacterMovementComponent|SetAirControlBoostMultiplier _charactermovement 2.0)
      (Variables|/Script/Engine.CharacterMovementComponent|SetAirControlBoostVelocityThreshold _charactermovement 25.0))
    (:Physic
      ;;[1 1 1] Reset physics objects
      (Class|PrimitiveComponent|SetLinearDamping (Actor|GetComponentbyClass (Variables|Default|GetResetActor) "/Script/Engine.StaticMeshComponent") 1.0)
      (Class|PrimitiveComponent|SetAngularDamping (Actor|GetComponentbyClass (Variables|Default|GetResetActor) "/Script/Engine.StaticMeshComponent") 2.0)
      (Class|PrimitiveComponent|AddVelocityChangeImpulseatLocation (Actor|GetComponentbyClass (Variables|Default|GetResetActor) "/Script/Engine.StaticMeshComponent") "0, 0, 0" "0, 0, 0" "None"))
    (:Timeline
      ;;[1 1 1] Reset mechanics using a Timeline
      (Variables|/Script/Engine.Actor|SetCustomTimeDilation (Variables|Default|GetResetActor) 1.0)))
  (Development|PrintString (Utilities|String|Append (Utilities|GetDisplayName (Variables|Default|GetResetActor)) " is reset") true true "(R=1.000000,G=0.000000,B=0.000000,A=1.000000)"))

(event Custom|AddEffect
  ;[1 1 1] À la création de la zone et à chaque fois qu'un object y entre, regarder chaque object pour voir ceux qui possèdent un Tag voulu. Retourne en string ce Tag, qui peut ensuite être accéder par les BP child des 3 zones pour déterminer comment l'object sera affecté par celles-ci
)

(event Custom|UpdateMain
  (bind _overlappingactors (Collision|GetOverlappingActors "/Script/Engine.Actor" :!class /Script/Engine.Actor))
  ;[1 1 1] À la création de la zone et à chaque fois qu'un object y entre, regarder chaque object pour voir ceux qui possèdent un Tag voulu. Retourne en string ce Tag, qui peut ensuite être accéder par les BP child des 3 zones pour déterminer comment l'object sera affecté par celles-ci
  (Variables|Default|SetOverlapping%20Actors _overlappingactors)
  (for (_ _array_index) _overlappingactors
    (Variables|Default|SetAffectedActor (Utilities|Array|Get(acopy) _overlappingactors _array_index))
    (bind _tag (CallFunction|CheckObjectTag (Variables|Default|GetAffectedActor)))
    (Variables|Default|SetAffectedActorTag _tag)
    (CallFunction|AddEffect)))

(event EventBeginPlay
  ;[1 1 1] À la création de la zone et à chaque fois qu'un object y entre, regarder chaque object pour voir ceux qui possèdent un Tag voulu. Retourne en string ce Tag, qui peut ensuite être accéder par les BP child des 3 zones pour déterminer comment l'object sera affecté par celles-ci
  (CallFunction|UpdateMain))

(event EventDestroyed
  ;[1 1 1] Lorsqu'on quitte la zone
)

(event EventTick
  (params (DeltaSeconds :type Float%20%28single-precision%29))
  ;[1 1 1] Lorsqu'on quitte la zone
  ;;[1 1 1] When deleted
)

(fn ConstructionScript)

(fn CheckObjectTag
  (params (ObjectToCheck :type Actor%20Object%20Reference))
  (if (Actor|ActorHasTag ObjectToCheck "Player")
    (return "Player" true)
    (elif (Actor|ActorHasTag ObjectToCheck "Physic")
      (return "Physic" true)
      (elif (Actor|ActorHasTag ObjectToCheck "Timeline")
        (return "Timeline" true)
        (else
          (return "" false))))))