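; Fast time zone, a child Blueprint that speeds up actors affected by it.
; It overrides AddEffect and switches on the affected actor's tag: Player, Physic and Timeline actors get doubled time dilation.
; The player also gets a set jump velocity, and physics objects get negative linear and zero angular damping.
; A debug print names the affected actor; leftover reset and walk speed nodes are disconnected.
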(event EventBeginPlay
  (|CallParentFunction))

(event Collision|EventActorBeginOverlap
  (params (OtherActor :type Actor%20Object%20Reference)))

(event Collision|EventActorEndOverlap
  (params (OtherActor :type Actor%20Object%20Reference))
  ;[1 1 1] Comment
)

(event EventAddEffect
  (bind _affectedactor (Variables|Default|GetAffectedActor))
  (bind _returnvalue (Actor|GetComponentbyClass _affectedactor "/Script/Engine.StaticMeshComponent"))
  (switch string (Variables|Default|GetAffectedActorTag)
    (:Player
      ;[1 1 1] Player
      (Variables|/Script/Engine.Actor|SetCustomTimeDilation (Variables|Default|GetAffectedActor) 2.0)
      (Variables|/Script/Engine.CharacterMovementComponent|SetJumpZVelocity (Variables|/Script/Engine.Character|GetCharacterMovement (Game|GetPlayerCharacter 0)) 8.4e+02))
    (:Physic
      ;[1 1 1] Pysics Objects
      (Class|PrimitiveComponent|SetLinearDamping _returnvalue -2.0)
      (Class|PrimitiveComponent|SetAngularDamping _returnvalue 0.0)
      (Variables|/Script/Engine.Actor|SetCustomTimeDilation (Variables|Default|GetAffectedActor) 2.0))
    (:Timeline
      ;[1 1 1] Mechanics using a Timeline
      (Variables|/Script/Engine.Actor|SetCustomTimeDilation (Variables|Default|GetAffectedActor) 2.0)))
  ;[1 1 1] Print
  (Development|PrintString (Utilities|String|Append (Utilities|GetDisplayName (Variables|Default|GetAffectedActor)) " affecté par " (Utilities|GetDisplayName self)) true true "(R=1.000000,G=1.000000,B=0.000000,A=1.000000)"))

(fn ConstructionScript
  (|CallParentFunction))