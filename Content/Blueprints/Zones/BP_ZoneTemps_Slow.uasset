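; Slow time zone Blueprint that overrides AddEffect to slow affected actors according to their tag.
; Players get reduced time dilation plus retuned jump, walk, gravity and air control on player character 0.
; Physics objects get heavy linear and angular damping with zero time dilation, while Timeline-driven mechanics just get reduced dilation.
; It prints each affected actor; its own overlap events are empty and its reset logic is disconnected.
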(event EventBeginPlay
  (|CallParentFunction))

(event Collision|EventActorBeginOverlap
  (params (OtherActor :type Actor%20Object%20Reference)))

(event EventAddEffect
  (bind _returnvalue (Game|GetPlayerCharacter 0))
  (bind _affectedactor (Variables|Default|GetAffectedActor))
  (bind _returnvalue_2 (Actor|GetComponentbyClass _affectedactor "/Script/Engine.StaticMeshComponent"))
  (bind _charactermovement (Variables|/Script/Engine.Character|GetCharacterMovement _returnvalue))
  (switch string (Variables|Default|GetAffectedActorTag)
    (:Player
      ;[1 1 1] Player
      (Variables|/Script/Engine.Actor|SetCustomTimeDilation (Variables|Default|GetAffectedActor) 0.25)
      (Variables|/Script/Engine.CharacterMovementComponent|SetJumpZVelocity _charactermovement 6e+02)
      (Variables|/Script/Engine.CharacterMovementComponent|SetMaxWalkSpeed _charactermovement 5e+02)
      (Variables|/Script/Engine.CharacterMovementComponent|SetGravityScale _charactermovement 4.0)
      (Variables|/Script/Engine.CharacterMovementComponent|SetAirControlBoostMultiplier _charactermovement 5e+01)
      (Variables|/Script/Engine.CharacterMovementComponent|SetAirControlBoostVelocityThreshold _charactermovement 4e+02))
    (:Physic
      ;[1 1 1] Pysics Objects
      (Class|PrimitiveComponent|SetLinearDamping _returnvalue_2 1e+01)
      (Class|PrimitiveComponent|SetAngularDamping _returnvalue_2 1e+01)
      (Variables|/Script/Engine.Actor|SetCustomTimeDilation (Variables|Default|GetAffectedActor) 0.0))
    (:Timeline
      ;[1 1 1] Mechanics using a Timeline
      (Variables|/Script/Engine.Actor|SetCustomTimeDilation (Variables|Default|GetAffectedActor) 0.3)))
  ;[1 1 1] Print
  (Development|PrintString (Utilities|String|Append (Utilities|GetDisplayName (Variables|Default|GetAffectedActor)) " affecté par " (Utilities|GetDisplayName self)) true true "(R=0.000000,G=0.000000,B=1.000000,A=1.000000)"))

(event Collision|EventActorEndOverlap
  (params (OtherActor :type Actor%20Object%20Reference))
  ;[1 1 1] Comment
)

(fn ConstructionScript
  (|CallParentFunction))