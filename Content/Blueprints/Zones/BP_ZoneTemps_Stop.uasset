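; BP_ZoneTemps_Stop is a child time-zone Blueprint that applies a stop effect to affected actors.
; AddEffect branches on actor tag: timelines drive the player's CustomTimeDilation and physics meshes' linear and angular damping, while Timeline-driven mechanics get zero dilation instantly.
; Both timelines abort if the affected actor matches OtherActorEnd, and debug prints report results.
; A player leaving the zone has their velocity zeroed; the ResetEffect call is unconnected.
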(event EventBeginPlay
  (|CallParentFunction))

(event Collision|EventActorBeginOverlap
  (params (OtherActor :type Actor%20Object%20Reference)))

(event EventTick
  (params (DeltaSeconds :type Float%20%28single-precision%29))
  (|CallParentFunction DeltaSeconds))

(event EventAddEffect
  (bind _affectedactor (Variables|Default|GetAffectedActor))
  (bind _returnvalue (Actor|GetComponentbyClass _affectedactor "/Script/Engine.StaticMeshComponent"))
  (switch string (Variables|Default|GetAffectedActorTag)
    (:Player
      ;[1 1 1] Player
      (bind _newtrack_1 (Timeline|Timeline_1-0/0,5sec Play)
        (:Update
          (if (!= (Variables|Default|GetAffectedActor) (Variables|Default|GetOther%20Actor_End))
            (Variables|/Script/Engine.Actor|SetCustomTimeDilation (Variables|Default|GetAffectedActor) _newtrack_1)
            (else
              (Variables|Default|SetOther%20Actor_End (Variables|Default|GetEmpty))
              (Development|PrintString "Early end" true true "(R=1.000000,G=0.000000,B=0.941978,A=1.000000)")
              (Timeline|Timeline_1-0/0,5sec Stop))))
        (:Finished
          ;[1 1 1] Print
          (Development|PrintString (Utilities|String|Append (Utilities|GetDisplayName (Variables|Default|GetAffectedActor)) " affecté par " (Utilities|GetDisplayName self)) true true "(R=0.300000,G=0.300000,B=0.300000,A=1.000000)" :!label _label))))
    (:Physic
      ;[1 1 1] Pysics Objects
      (bind _newtrack_1_2 (Timeline|Timeline_5-60-1000/1sec Play)
        (:Update
          (if (!= (Variables|Default|GetAffectedActor) (Variables|Default|GetOther%20Actor_End))
            (Class|PrimitiveComponent|SetLinearDamping _returnvalue _newtrack_1_2)
            (Class|PrimitiveComponent|SetAngularDamping _returnvalue _newtrack_1_2)
            (else
              (Variables|Default|SetOther%20Actor_End (Variables|Default|GetEmpty))
              (Development|PrintString "Early end" true true "(R=1.000000,G=0.000000,B=0.941978,A=1.000000)")
              (Timeline|Timeline_5-60-1000/1sec Stop))))
        (:Finished
          (goto _label))))
    (:Timeline
      ;[1 1 1] Mechanics using a Timeline
      (Variables|/Script/Engine.Actor|SetCustomTimeDilation (Variables|Default|GetAffectedActor) 0.0)
      (goto _label))))

(event Collision|EventActorEndOverlap
  (params (OtherActor :type Actor%20Object%20Reference))
  ;[1 1 1] Comment
  (if (Actor|ActorHasTag OtherActor "Player")
    (Variables|/Script/Engine.MovementComponent|SetVelocity (Variables|/Script/Engine.Character|GetCharacterMovement (Game|GetPlayerCharacter 0)) "0, 0, 0")))

(fn ConstructionScript
  (|CallParentFunction))