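; ChronoCanon weapon attached to the first-person player that shoots Slow, Fast or Stop time zones, with Fast and Stop unlocked by modules.
; Line-trace shots spawn zones attached to the hit component or replace a targeted zone, delayed by distance.
; Parallel zone and parent arrays track limited charges, recycling the oldest when empty; a delete laser refunds charges.
; Tick updates gun material and HUD tags, handles player resets, and blocks use while grabbing.
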(event Input|EnhancedActionEvents|EnhancedInputActionIA_Shoot
  (params (ActionValue :type Boolean) (ElapsedSeconds :type Float%20%28double-precision%29) (TriggeredSeconds :type Float%20%28double-precision%29) (InputAction :type Input%20Action%20Object%20Reference :default "/Game/FirstPerson/Input/Actions/IA_Shoot.IA_Shoot"))
  (bind _player (Variables|Default|GetPlayer))
  (bind _firstpersoncamera (Variables|/Game/FirstPerson/Blueprints/BP_FirstPersonCharacter.BP_FirstPersonCharacter_C|GetFirstPersonCamera _player))
  (bind _returnvalue (Transformation|GetWorldLocation _firstpersoncamera))
  ;[1 1 1] Lorsque le joueur tire, ça tire un line trace et joue l'animation de tire
  (:Triggered
    (bind _outhit (CallFunction|Fire _returnvalue (+ _returnvalue (* (Math|Vector|GetForwardVector (Transformation|GetWorldRotation _firstpersoncamera)) (Variables|Default|GetMaxDistance)))))
    (Variables|Default|SetHitLocation (.Location (Collision|BreakHitResult _outhit)))
    (Animation|Montage|MontagePlay (Components|SkeletalMesh|GetAnimInstance (Variables|/Game/FirstPerson/Blueprints/BP_FirstPersonCharacter.BP_FirstPersonCharacter_C|GetFirstPersonMesh (Variables|Default|GetPlayer))) "/Game/FirstPersonArms/Animations/FP_Rifle_Shoot_Montage.FP_Rifle_Shoot_Montage" 1.0 "MontageLength" 0.0 false)
    ;[1 1 1] Le FX du laser apprait à dans la location voulu.
    (Game|SpawnActorfromClass "/Game/Blueprints/Mechaniques/Laser/BP_LaserFX_Place.BP_LaserFX_Place_C" (Math|Conversions|ToTransform(Vector) (Transformation|GetSocketLocation "Barrel")) "Undefined" 0 0)
    ;[1 1 1] Ajoute l'information des actors et components hit par le line trace
    (Variables|Default|SetHitComponent (.HitComponent (Collision|BreakHitResult _outhit)))
    (bind _output_get (Variables|Default|SetHit%20Actor (.HitActor (Collision|BreakHitResult _outhit))))
    ;[1 1 1] Vérifie si le hit actor a les tags Untargetable ou Zone
    (Utilities|IsValid _output_get
      (:Is%20Valid
        (if (Actor|ActorHasTag _output_get "Untargetable")
          (Development|PrintString "Untargetable")
          (elif (Actor|ActorHasTag _output_get "Zone")
            (Utilities|FlowControl|Delay (/ (.Distance (Collision|BreakHitResult _outhit)) 7e+03))
            ;[1 1 1] Détermine quel type de zone à remplacer avec
            (switch int (Variables|Default|GetZoneType)
              (:0
                (CallFunction|ReplaceSlow (Math|Conversions|ToTransform(Vector) (Transformation|GetWorldLocation (.HitComponent (Collision|BreakHitResult _outhit))))))
              (:1
                (CallFunction|ReplaceFast (Math|Conversions|ToTransform(Vector) (Transformation|GetWorldLocation (.HitComponent (Collision|BreakHitResult _outhit))))))
              (:2
                (CallFunction|ReplaceStop (Math|Conversions|ToTransform(Vector) (Transformation|GetWorldLocation (.HitComponent (Collision|BreakHitResult _outhit)))))))
            (Utilities|FlowControl|Delay 0.2)
            (Variables|Default|SetIsDelay false)
            (else
              ;[1 1 1] Vérifie si le joueur n'a plus de charges, si oui joue la fonction correspondante
              (if (Variables|Default|GetIsOutOfCharges)
                (Development|PrintString "Function Called OOC")
                (CallFunction|OutOfCharges))
              (Utilities|FlowControl|Delay (/ (.Distance (Collision|BreakHitResult _outhit)) 7e+03))
              ;[1 1 1] Détermine quel type de zone a spawner.
              (switch int (Variables|Default|GetZoneType)
                (:0
                  (CallFunction|SpawnSlow (Math|Conversions|ToTransform(Vector) (.Location (Collision|BreakHitResult _outhit)))))
                (:1
                  (CallFunction|SpawnFast (Math|Conversions|ToTransform(Vector) (.Location (Collision|BreakHitResult _outhit)))))
                (:2
                  (CallFunction|SpawnStop (Math|Conversions|ToTransform(Vector) (.Location (Collision|BreakHitResult _outhit))))))
              (Utilities|FlowControl|Delay 0.2)
              (Variables|Default|SetIsDelay false))))))))

(event Input|EnhancedActionEvents|EnhancedInputActionIA_ZoneDelete
  (params (ActionValue :type Boolean) (ElapsedSeconds :type Float%20%28double-precision%29) (TriggeredSeconds :type Float%20%28double-precision%29) (InputAction :type Input%20Action%20Object%20Reference :default "/Game/FirstPerson/Input/Actions/IA_ZoneDelete.IA_ZoneDelete"))
  (bind _maxdistance (Variables|Default|GetMaxDistance))
  (bind _zonesarray (Variables|Default|GetZonesArray))
  (bind _parentarray (Variables|Default|GetParentArray))
  (bind _out_hit_hit_actor (Variables|Default|GetOut%20Hit%20Hit%20Actor))
  (bind _out_hit_hit_actor_2 (Variables|Default|GetOut%20Hit%20Hit%20Actor))
  (bind _player (Variables|Default|GetPlayer))
  (bind _firstpersoncamera (Variables|/Game/FirstPerson/Blueprints/BP_FirstPersonCharacter.BP_FirstPersonCharacter_C|GetFirstPersonCamera _player))
  (bind _returnvalue (Transformation|GetWorldLocation _firstpersoncamera))
  (bind _returnvalue_2 (Transformation|GetWorldRotation _firstpersoncamera))
  (bind _returnvalue_3 (Math|Vector|GetForwardVector _returnvalue_2))
  (bind _returnvalue_4 (* _returnvalue_3 _maxdistance))
  (bind _returnvalue_5 (+ _returnvalue _returnvalue_4))
  (:Triggered
    (Variables|Default|SetTraceEnd _returnvalue_5)
    (if (not (Variables|Default|GetIsGrabbing))
      ;[1 0.1648 0] Le line trace et Niagara FX qui sont fusionné
      (bind (_niagara_output_laser _niagara_output_laser_impact) (CallFunction|ZoneLineTraceVFX (Math|Conversions|ToTransform(Vector) (Transformation|GetSocketLocation "Barrel")) _returnvalue _returnvalue_5))
      (Variables|Default|SetNiagara%20Output%20Laser _niagara_output_laser)
      (Variables|Default|SetNiagara%20Output%20Laser%20Impact _niagara_output_laser_impact)
      ;[1 0 0.08404] Animation du fusil
      (Animation|Montage|MontagePlay (Components|SkeletalMesh|GetAnimInstance (Variables|/Game/FirstPerson/Blueprints/BP_FirstPersonCharacter.BP_FirstPersonCharacter_C|GetFirstPersonMesh (Variables|Default|GetPlayer))) "/Game/FirstPersonArms/Animations/FP_Rifle_Shoot_Montage.FP_Rifle_Shoot_Montage" 1.0 "MontageLength" 0.0 true)
      ;[1 0 0.09349] Le son quand le joueur tire.
      (Audio|PlaySound2D "/Game/Sounds/Gun/Gun_shot_Delete.Gun_shot_Delete" 1.0 1.0 0.0 0 0)
      ;[1 1 1] Vérifie si le hit actor est une zone avant de détruire l'actor
      (if (not (Variables|Default|GetIsShooting))
        (Utilities|IsValid _out_hit_hit_actor
          (:Is%20Valid
            (if (Actor|ActorHasTag _out_hit_hit_actor "Zone")
              ;[1 1 1] Si le actor est une zone, on l'enlève de l'array, et on enlève son parent du parentarray
              (bind _output_get (Variables|Default|SetIndexReplace (Utilities|Array|FindItem _zonesarray _out_hit_hit_actor_2)))
              (Utilities|Array|RemoveItem _parentarray (Utilities|Array|Get(acopy) _parentarray _output_get))
              (Utilities|Array|RemoveItem _zonesarray _out_hit_hit_actor_2)
              ;[1 1 1] Détruit la zone et regagne une charge
              (Actor|DestroyActor (Variables|Default|GetOut%20Hit%20Hit%20Actor))
              (Variables|Default|SetCharges (+ (Variables|Default|GetCharges) 1))
              (else
                (Development|PrintString "Not a zone")))))))))

(event Input|EnhancedActionEvents|EnhancedInputActionIA_ZoneSlow
  (params (ActionValue :type Boolean) (ElapsedSeconds :type Float%20%28double-precision%29) (TriggeredSeconds :type Float%20%28double-precision%29) (InputAction :type Input%20Action%20Object%20Reference :default "/Game/FirstPerson/Input/Actions/IA_ZoneSlow.IA_ZoneSlow"))
  ;[1 1 1] Change le type de zone du ChronoCanon a Slow
  (:Triggered
    (if (not (Variables|Default|GetIsGrabbing))
      (Variables|Default|SetZoneType 0)
      (Audio|PlaySound2D "/Game/Sounds/Gun/Changement_Gun/Changement_Gun_1.Changement_Gun_1" 1.0 1.0 0.0 0 0))))

(event Input|EnhancedActionEvents|EnhancedInputActionIA_ZoneAccelere
  (params (ActionValue :type Boolean) (ElapsedSeconds :type Float%20%28double-precision%29) (TriggeredSeconds :type Float%20%28double-precision%29) (InputAction :type Input%20Action%20Object%20Reference :default "/Game/FirstPerson/Input/Actions/IA_ZoneAccelere.IA_ZoneAccelere"))
  ;[1 1 1] Change le type de zone du ChronoCanon a Fast
  (:Triggered
    (if (not (Variables|Default|GetIsGrabbing))
      (if (Variables|Default|GetFastActive?)
        (Variables|Default|SetZoneType 1)
        (Audio|PlaySound2D "/Game/Sounds/Gun/Changement_Gun/Changement_Gun_3.Changement_Gun_3" 1.0 1.0 0.0 0 0)))))

(event Input|EnhancedActionEvents|EnhancedInputActionIA_ZoneStop
  (params (ActionValue :type Boolean) (ElapsedSeconds :type Float%20%28double-precision%29) (TriggeredSeconds :type Float%20%28double-precision%29) (InputAction :type Input%20Action%20Object%20Reference :default "/Game/FirstPerson/Input/Actions/IA_ZoneStop.IA_ZoneStop"))
  ;[1 1 1] Change le type de zone du ChronoCanon a Stop
  (:Triggered
    (if (not (Variables|Default|GetIsGrabbing))
      (if (Variables|Default|GetStopActive?)
        (Variables|Default|SetZoneType 2)
        (Audio|PlaySound2D "/Game/Sounds/Gun/Changement_Gun/Changement_Gun_2.Changement_Gun_2" 1.0 1.0 0.0 0 0)))))

(event Input|EnhancedActionEvents|EnhancedInputActionIA_ChangementScrollUp
  (params (ActionValue :type Boolean) (ElapsedSeconds :type Float%20%28double-precision%29) (TriggeredSeconds :type Float%20%28double-precision%29) (InputAction :type Input%20Action%20Object%20Reference :default "/Game/FirstPerson/Input/Actions/IA_ChangementScrollUp.IA_ChangementScrollUp"))
  ;[1 1 1] Change le type de zone
  (:Triggered
    (if (not (Variables|Default|GetIsGrabbing))
      (if (Variables|Default|GetFastActive?)
        (if (Variables|Default|GetStopActive?)
          (if (== (Variables|Default|GetZoneType) 2)
            (Variables|Default|SetZoneType 0)
            (else
              (Variables|Default|SetZoneType (+ (Variables|Default|GetZoneType) 1))))
          (Audio|PlaySound2D "/Game/Sounds/Gun/Changement_Gun/Changement_Gun_cue.Changement_Gun_cue" 1.0 1.0 0.0 0 0)
          (else
            (if (== (Variables|Default|GetZoneType) 1)
              (Variables|Default|SetZoneType 0)
              (else
                (Variables|Default|SetZoneType (+ (Variables|Default|GetZoneType) 1))))
            (Audio|PlaySound2D "/Game/Sounds/Gun/Changement_Gun/Changement_Gun_cue.Changement_Gun_cue" 1.0 1.0 0.0 0 0)))
        (else
          (Development|PrintString "Module Missing"))))))

(event Input|EnhancedActionEvents|EnhancedInputActionIA_ChangementScrollDown
  (params (ActionValue :type Boolean) (ElapsedSeconds :type Float%20%28double-precision%29) (TriggeredSeconds :type Float%20%28double-precision%29) (InputAction :type Input%20Action%20Object%20Reference :default "/Game/FirstPerson/Input/Actions/IA_ChangementScrollDown.IA_ChangementScrollDown"))
  ;[1 1 1] Change le type de zone
  (:Triggered
    (if (not (Variables|Default|GetIsGrabbing))
      (if (Variables|Default|GetFastActive?)
        (if (Variables|Default|GetStopActive?)
          (if (== (Variables|Default|GetZoneType) 0)
            (Variables|Default|SetZoneType 2)
            (else
              (Variables|Default|SetZoneType (- (Variables|Default|GetZoneType) 1))))
          (Audio|PlaySound2D "/Game/Sounds/Gun/Changement_Gun/Changement_Gun_cue.Changement_Gun_cue" 1.0 1.0 0.0 0 0)
          (else
            (if (== (Variables|Default|GetZoneType) 0)
              (Variables|Default|SetZoneType 1)
              (else
                (Variables|Default|SetZoneType 0)))
            (Audio|PlaySound2D "/Game/Sounds/Gun/Changement_Gun/Changement_Gun_cue.Changement_Gun_cue" 1.0 1.0 0.0 0 0)))))))

(event EventBeginPlay
  (bind _player (Variables|Default|GetPlayer))
  (Development|PrintString "Attached")
  ;[1 1 1] Attache le SKM au joueur
  (CallFunction|AttachWeapon)
  ;[1 1 1] Ajoute les contrôles du ChronoCanon au joueur et set l'animation du ChronoCanon
  (Variables|/Game/FirstPerson/Blueprints/BP_FirstPersonCharacter.BP_FirstPersonCharacter_C|SetbHasRifle _player true)
  (bind _asplayer_controller (Utilities|Casting|CastToPlayerController (Pawn|GetController _player)))
  (Utilities|IsValid (PlayerController|LocalPlayerSubsystems|GetEnhancedInputLocalPlayerSubsystem _asplayer_controller)
    (:Is%20Valid
      (Input|AddMappingContext (PlayerController|LocalPlayerSubsystems|GetEnhancedInputLocalPlayerSubsystem _asplayer_controller) "/Game/FirstPerson/Input/IMC_Weapons.IMC_Weapons" 0 "(bIgnoreAllPressedKeysUntilRelease=True,bForceImmediately=False)"))))

(event EventTick
  (params (DeltaSeconds :type Float%20%28single-precision%29))
  (bind _player (Variables|Default|GetPlayer))
  (bind _player_2 (Variables|Default|GetPlayer))
  ;[1 1 1] Reset tout les zones que le joueur a générées lorsque le joueur meurt
  (if (Variables|/Game/FirstPerson/Blueprints/BP_FirstPersonCharacter.BP_FirstPersonCharacter_C|GetResetZones _player)
    (Utilities|Array|Clear (Variables|Default|GetZonesArray))
    (Utilities|Array|Clear (Variables|Default|GetParentArray))
    (Variables|Default|SetCharges 3)
    (Variables|/Game/FirstPerson/Blueprints/BP_FirstPersonCharacter.BP_FirstPersonCharacter_C|SetResetZones _player false))
  (CallFunction|VerificationCube)
  ;[1 1 1] Calcule la charge du joueur
  (CallFunction|CalculeCharge)
  ;[1 1 1] Change la texture du ChronoCanon dépandament du zone
  (CallFunction|ChangementDeCouleur)
  ;[1 1 1] Envoie l'information du type de zone au HUD
  (Variables|/Game/FirstPerson/Blueprints/BP_FirstPersonCharacter.BP_FirstPersonCharacter_C|SetZoneType _player_2 (Variables|Default|GetZoneType))
  (CallFunction|SetZonesHUD _player_2)
  ;[1 1 1] Change le bool pour activer les fonctions de zone rapide et stop quand le joueur prends les modules respectifs
  (if (Variables|/Game/FirstPerson/Blueprints/BP_FirstPersonCharacter.BP_FirstPersonCharacter_C|GetHasStop _player_2)
    (Variables|Default|SetStopActive? true))
  (if (Variables|/Game/FirstPerson/Blueprints/BP_FirstPersonCharacter.BP_FirstPersonCharacter_C|GetHasSpeed _player_2)
    (Variables|Default|SetFastActive? true)))

(fn CalculeCharge
  ;[1 1 1] Détermine si il reste 0 charges au joueur
  (if (== (Variables|Default|GetCharges) 0)
    (Variables|Default|SetIsOutOfCharges true)
    (else
      (Variables|Default|SetIsOutOfCharges false))))

(fn SpawnStop
  (params (SpawnTransform :type Transform))
  (bind _hitcomponent (Variables|Default|GetHitComponent))
  ;[1 1 1] Spawn la zone et l'attache au component qu'il a hit pour que la zone puisse bouger avec ex: piston et plateforme. Ajoute aussi un tag pour identifier la zone comme zone générée par le joueur.
  (bind _returnvalue (Game|SpawnActorfromClass "/Game/Blueprints/Zones/BP_ZoneTemps_Stop.BP_ZoneTemps_Stop_C" SpawnTransform "Undefined" (Variables|Default|GetHit%20Actor) (Variables|Default|GetPlayer)))
  (Utilities|Array|Add (Variables|/Script/Engine.Actor|GetTags _returnvalue) "PlayerZone")
  (Transformation|AttachComponentToComponent _returnvalue _hitcomponent "None" "KeepWorld" "KeepWorld" "KeepWorld" true)
  ;[1 1 1] Ajoute la zone dans la zone array et ajoute son parent dans un autre array.
  (Utilities|Array|Add (Variables|Default|GetZonesArray) _returnvalue)
  (Utilities|Array|Add (Variables|Default|GetParentArray) _hitcomponent)
  ;[1 1 1] Enlève la charge après le tir est change l'état a du tir a faux
  (Variables|Default|SetCharges (- (Variables|Default|GetCharges) 1))
  (Variables|Default|SetIsShooting false)
  (Variables|Default|SetIsDelay true))

(fn SpawnFast
  (params (SpawnTransform :type Transform))
  (bind _hitcomponent (Variables|Default|GetHitComponent))
  ;[1 1 1] Spawn la zone et l'attache au component qu'il a hit pour que la zone puisse bouger avec ex: piston et plateforme. Ajoute aussi un tag pour identifier la zone comme zone générée par le joueur.
  (bind _returnvalue (Game|SpawnActorfromClass "/Game/Blueprints/Zones/BP_ZoneTemps_Fast.BP_ZoneTemps_Fast_C" SpawnTransform "Undefined" 0 (Variables|Default|GetPlayer)))
  (Utilities|Array|Add (Variables|/Script/Engine.Actor|GetTags _returnvalue) "PlayerZone")
  (Transformation|AttachComponentToComponent _returnvalue _hitcomponent "None" "KeepWorld" "KeepWorld" "KeepWorld" true)
  ;[1 1 1] Ajoute la zone dans la zone array et ajoute son parent dans un autre array.
  (Utilities|Array|Add (Variables|Default|GetZonesArray) _returnvalue)
  (Utilities|Array|Add (Variables|Default|GetParentArray) _hitcomponent)
  ;[1 1 1] Enlève la charge après le tir est change l'état a du tir a faux
  (Variables|Default|SetCharges (- (Variables|Default|GetCharges) 1))
  (Variables|Default|SetIsShooting false)
  (Variables|Default|SetIsDelay true))

(fn SpawnSlow
  (params (SpawnTransform :type Transform))
  (bind _hitcomponent (Variables|Default|GetHitComponent))
  ;[1 1 1] Spawn la zone et l'attache au component qu'il a hit pour que la zone puisse bouger avec ex: piston et plateforme. Ajoute aussi un tag pour identifier la zone comme zone générée par le joueur.
  (bind _returnvalue (Game|SpawnActorfromClass "/Game/Blueprints/Zones/BP_ZoneTemps_Slow.BP_ZoneTemps_Slow_C" SpawnTransform "Undefined" (Variables|Default|GetHit%20Actor) (Variables|Default|GetPlayer)))
  (Utilities|Array|Add (Variables|/Script/Engine.Actor|GetTags _returnvalue) "PlayerZone")
  (Transformation|AttachComponentToComponent _returnvalue _hitcomponent "None" "KeepWorld" "KeepWorld" "KeepWorld" true)
  ;[1 1 1] Ajoute la zone dans la zone array et ajoute son parent dans un autre array.
  (Utilities|Array|Add (Variables|Default|GetZonesArray) _returnvalue)
  (Utilities|Array|Add (Variables|Default|GetParentArray) _hitcomponent)
  ;[1 1 1] Enlève la charge après le tir est change l'état a du tir a faux
  (Variables|Default|SetCharges (- (Variables|Default|GetCharges) 1))
  (Variables|Default|SetIsShooting false)
  (Variables|Default|SetIsDelay true))

(fn ReplaceSlow
  (params (SpawnTransform :type Transform))
  (bind _hit_actor (Variables|Default|GetHit%20Actor))
  (bind _zonesarray (Variables|Default|GetZonesArray))
  ;[1 1 1] Cherche est replace la zone tirée par la nouvelle dans le array
  (Variables|Default|SetIndexReplace (Utilities|Array|FindItem _zonesarray _hit_actor))
  (Utilities|Array|RemoveItem _zonesarray _hit_actor)
  (if (Actor|ActorHasTag _hit_actor "Zone")
    (Actor|DestroyActor _hit_actor)
    ;[1 1 1] Génére la nouvelle zone est l'attache sur le parent de la zone ancienne, ajoute un tag pour l'identifiée comme
    (bind _returnvalue (Game|SpawnActorfromClass "/Game/Blueprints/Zones/BP_ZoneTemps_Slow.BP_ZoneTemps_Slow_C" SpawnTransform "Undefined" 0 (Variables|Default|GetPlayer)))
    (Utilities|Array|Add (Variables|/Script/Engine.Actor|GetTags _returnvalue) "PlayerZone")
    (Transformation|AttachComponentToComponent _returnvalue (Utilities|Array|Get(acopy) (Variables|Default|GetParentArray) (Variables|Default|GetIndexReplace)) "None" "KeepWorld" "KeepWorld" "KeepWorld" true)
    ;[1 1 1] Ajoute la nouvelle zone dans le zone array
    (Utilities|Array|Add (Variables|Default|GetZonesArray) _returnvalue)
    (Variables|Default|SetIsShooting false)
    (Variables|Default|SetIsDelay true)))

(fn ReplaceFast
  (params (SpawnTransform :type Transform))
  (bind _hit_actor (Variables|Default|GetHit%20Actor))
  (bind _zonesarray (Variables|Default|GetZonesArray))
  ;[1 1 1] Cherche est replace la zone tirée par la nouvelle dans le array
  (Variables|Default|SetIndexReplace (Utilities|Array|FindItem _zonesarray _hit_actor))
  (Utilities|Array|RemoveItem _zonesarray _hit_actor)
  (if (Actor|ActorHasTag _hit_actor "Zone")
    (Actor|DestroyActor _hit_actor)
    ;[1 1 1] Génére la nouvelle zone est l'attache sur le parent de la zone ancienne, ajoute un tag pour l'identifiée comme
    (bind _returnvalue (Game|SpawnActorfromClass "/Game/Blueprints/Zones/BP_ZoneTemps_Fast.BP_ZoneTemps_Fast_C" SpawnTransform "Undefined" 0 (Variables|Default|GetPlayer)))
    (Utilities|Array|Add (Variables|/Script/Engine.Actor|GetTags _returnvalue) "PlayerZone")
    (Transformation|AttachComponentToComponent _returnvalue (Utilities|Array|Get(acopy) (Variables|Default|GetParentArray) (Variables|Default|GetIndexReplace)) "None" "KeepWorld" "KeepWorld" "KeepWorld" true)
    ;[1 1 1] Ajoute la nouvelle zone dans le zone array
    (Utilities|Array|Add (Variables|Default|GetZonesArray) _returnvalue)
    (Variables|Default|SetIsShooting false)
    (Variables|Default|SetIsDelay true)))

(fn ReplaceStop
  (params (SpawnTransform :type Transform))
  (bind _hit_actor (Variables|Default|GetHit%20Actor))
  (bind _zonesarray (Variables|Default|GetZonesArray))
  ;[1 1 1] Cherche est replace la zone tirée par la nouvelle dans le array
  (Variables|Default|SetIndexReplace (Utilities|Array|FindItem _zonesarray _hit_actor))
  (Utilities|Array|RemoveItem _zonesarray _hit_actor)
  (if (Actor|ActorHasTag _hit_actor "Zone")
    (Actor|DestroyActor _hit_actor)
    ;[1 1 1] Génére la nouvelle zone est l'attache sur le parent de la zone ancienne, ajoute un tag pour l'identifiée comme
    (bind _returnvalue (Game|SpawnActorfromClass "/Game/Blueprints/Zones/BP_ZoneTemps_Stop.BP_ZoneTemps_Stop_C" SpawnTransform "Undefined" (Variables|Default|GetHit%20Actor) (Variables|Default|GetPlayer)))
    (Utilities|Array|Add (Variables|/Script/Engine.Actor|GetTags _returnvalue) "PlayerZone")
    (Transformation|AttachComponentToComponent _returnvalue (Utilities|Array|Get(acopy) (Variables|Default|GetParentArray) (Variables|Default|GetIndexReplace)) "None" "KeepWorld" "KeepWorld" "KeepWorld" true)
    ;[1 1 1] Ajoute la nouvelle zone dans le zone array
    (Utilities|Array|Add (Variables|Default|GetZonesArray) _returnvalue)
    (Variables|Default|SetIsShooting false)
    (Variables|Default|SetIsDelay true)))

(fn OutOfCharges
  (bind _zonesarray (Variables|Default|GetZonesArray))
  ;[1 1 1] Identifie la zone la plus ancienne et l'enlève du array et le destroy, ensuite ajoute une charge au joueur.
  (Utilities|IsValid (Utilities|Array|Get(acopy) _zonesarray (Variables|Default|GetIndexNumber))
    (:Is%20Valid
      (Development|PrintString (Utilities|GetDisplayName (Utilities|Array|Get(acopy) _zonesarray (Variables|Default|GetIndexNumber))))
      (Actor|DestroyActor (Utilities|Array|Get(acopy) _zonesarray (Variables|Default|GetIndexNumber))))
    (:Is%20Not%20Valid
      _))
  (Utilities|Array|RemoveItem _zonesarray (Utilities|Array|Get(acopy) _zonesarray (Variables|Default|GetIndexNumber)))
  (Variables|Default|SetIndexNumber 0)
  (Variables|Default|SetCharges 1))

(fn ChangementDeCouleur
  ;[1 1 1] Change la texture du ChronoCanon selon le type de zone.
  (switch int (Variables|Default|GetZoneType)
    (:0
      (Rendering|Material|SetMaterial 0 "/Game/Assets/ChronoCanon/M_ChronoCanon.M_ChronoCanon"))
    (:1
      (Rendering|Material|SetMaterial 0 "/Game/Assets/ChronoCanon/M_ChronoCanon_22.M_ChronoCanon_22"))
    (:2
      (Rendering|Material|SetMaterial 0 "/Game/Assets/ChronoCanon/M_ChronoCanon33.M_ChronoCanon33"))))

(fn VerificationCube
  (bind _player (Variables|Default|GetPlayer))
  ;[1 1 1] Verifie si le joueur prend un cube, et désactive le ChronoCanon au besoin.
  (if (Variables|/Game/FirstPerson/Blueprints/BP_FirstPersonCharacter.BP_FirstPersonCharacter_C|GetIsGrabbing _player)
    (Variables|/Game/FirstPerson/Blueprints/BP_FirstPersonCharacter.BP_FirstPersonCharacter_C|SetbHasRifle _player false)
    (Variables|Default|SetIsGrabbing true)
    (else
      (Variables|Default|SetIsGrabbing false)
      (Variables|/Game/FirstPerson/Blueprints/BP_FirstPersonCharacter.BP_FirstPersonCharacter_C|SetbHasRifle _player true))))

(fn AttachWeapon
  ;[1 1 1] Attache le ChronoCanon à la main du joueur
  (bind _asbp_first_person_character (Utilities|Casting|CastToBP_FirstPersonCharacter (Components|GetOwner)))
  (Variables|/Game/FirstPerson/Blueprints/BP_FirstPersonCharacter.BP_FirstPersonCharacter_C|SetHasChronoCanon? _asbp_first_person_character true)
  (bind _output_get (Variables|Default|SetPlayer _asbp_first_person_character))
  (Transformation|AttachComponentToComponent (Variables|/Game/FirstPerson/Blueprints/BP_FirstPersonCharacter.BP_FirstPersonCharacter_C|GetFirstPersonMesh _output_get) "GripPoint" "SnapToTarget" "SnapToTarget" "SnapToTarget" true))

(fn Fire
  (params (LineStart :type Vector) (LineEnd :type Vector))
  ;[1 1 1] Verifie que les conditions sont respectées, et tire un line trace.
  (if (not (Variables|Default|GetIsGrabbing))
    (if (Variables|Default|GetIsDelay)
      _
      (else
        (Variables|Default|SetIsShooting true)
        (bind _outhit (Collision|LineTraceByChannel LineStart LineEnd "TraceTypeQuery2" false 0 "ForDuration"))
        (Audio|PlaySound2D "/Game/Sounds/Gun/Gun_shot.Gun_shot" 1.0 1.0 0.0 0 0)))
    (return 0 _outhit)))

(fn PlayAnim
  (params (Hit%20Actor :type Actor%20Object%20Reference) (HitComponent :type Primitive%20Component%20Object%20Reference) (self2 :type BP%20First%20Person%20Character%20Object%20Reference) (InputPin :type Vector))
  ;[1 1 1] Joue l'animation de tire, et set des variables du hit result provenant du line trace
  (Variables|Default|SetHitLocation InputPin)
  (Animation|Montage|MontagePlay (Components|SkeletalMesh|GetAnimInstance (Variables|/Game/FirstPerson/Blueprints/BP_FirstPersonCharacter.BP_FirstPersonCharacter_C|GetFirstPersonMesh self2)) "/Game/FirstPersonArms/Animations/FP_Rifle_Shoot_Montage.FP_Rifle_Shoot_Montage" 1.0 "MontageLength" 0.0 false)
  (Variables|Default|SetHitComponent HitComponent)
  (return 0))

(fn SetZonesHUD
  (params (self2 :type BP%20First%20Person%20Character%20Object%20Reference))
  (bind _zonesarray (Variables|Default|GetZonesArray))
  (bind _tagsarray (Variables|/Game/FirstPerson/Blueprints/BP_FirstPersonCharacter.BP_FirstPersonCharacter_C|GetTagsArray self2))
  (bind _output (Utilities|Array|Get(acopy) _zonesarray 2))
  (bind _output_2 (Utilities|Array|Get(acopy) _zonesarray))
  (bind _output_3 (Utilities|Array|Get(acopy) _zonesarray 1))
  (Utilities|IsValid _output_2
    (:Is%20Valid
      ;[1 1 1] Si le array index n'a pas de zone,  il met le tag array a else pour indiquer de rendre le cercle vide, sinon on donne le type de zone
      (Utilities|Array|SetArrayElem _tagsarray 0 (Utilities|Array|Get(acopy) (Variables|/Script/Engine.Actor|GetTags _output_2) 1)))
    (:Is%20Not%20Valid
      (Utilities|Array|SetArrayElem _tagsarray 0 "else")))
  (Utilities|IsValid _output_3
    (:Is%20Valid
      (Utilities|Array|SetArrayElem _tagsarray 1 (Utilities|Array|Get(acopy) (Variables|/Script/Engine.Actor|GetTags _output_3) 1)))
    (:Is%20Not%20Valid
      (Utilities|Array|SetArrayElem _tagsarray 1 "else")))
  (Utilities|IsValid _output
    (:Is%20Valid
      (Utilities|Array|SetArrayElem _tagsarray 2 (Utilities|Array|Get(acopy) (Variables|/Script/Engine.Actor|GetTags _output) 1)))
    (:Is%20Not%20Valid
      (Utilities|Array|SetArrayElem _tagsarray 2 "else"))))

(fn ZoneLineTraceVFX
  (params (SpawnTransform :type Transform) (Start :type Vector) (End :type Vector))
  (bind _outhit (Collision|LineTraceByChannel Start End "TraceTypeQuery3" false (Utilities|Array|MakeArray (Variables|Default|GetBP_Vitre)) "None"))
  ;[1 1 1] Déclaration de variable du hit et de la location de celui-ci.
  (Variables|Default|SetHit (.bblockinghit _outhit))
  (Variables|Default|SetOut%20Hit%20Location (.location _outhit))
  (Variables|Default|SetOut%20Hit%20Hit%20Actor (.hitactor _outhit))
  ;[1 1 1] Le FX du laser apprait à dans la location voulu.
  (bind _returnvalue (Game|SpawnActorfromClass "/Game/Blueprints/Mechaniques/Laser/BP_LaserFX_GunDelete.BP_LaserFX_GunDelete_C" (Math|Conversions|ToTransform(Vector) (Transformation|GetSocketLocation "Barrel")) "Undefined" 0 0))
  (bind _output_get (Variables|Default|SetLaserAsset _returnvalue))
  (Variables|/Game/Blueprints/Mechaniques/Laser/BP_LaserFX_GunDelete.BP_LaserFX_GunDelete_C|SetLaser_End _output_get (select (Variables|Default|GetHit) (Variables|Default|GetOut%20Hit%20Location) (Variables|Default|GetTraceEnd)))
  (Variables|/Game/Blueprints/Mechaniques/Laser/BP_LaserFX_GunDelete.BP_LaserFX_GunDelete_C|SetHit_Location _output_get (Variables|Default|GetOut%20Hit%20Location))
  (Variables|/Game/Blueprints/Mechaniques/Laser/BP_LaserFX_GunDelete.BP_LaserFX_GunDelete_C|SetHit _output_get (Variables|Default|GetHit))
  ;[1 1 1] La visibilité du FX est désactivé pour le moment.
  (Rendering|SetVisibility (Variables|/Game/Blueprints/Mechaniques/Laser/BP_LaserFX_GunDelete.BP_LaserFX_GunDelete_C|GetNiagaraLaser _output_get) true false)
  (return (Variables|/Game/Blueprints/Mechaniques/Laser/BP_LaserFX_GunDelete.BP_LaserFX_GunDelete_C|GetNiagaraLaser _output_get) (Variables|/Game/Blueprints/Mechaniques/Laser/BP_LaserFX_GunDelete.BP_LaserFX_GunDelete_C|GetNiagaraLaserImpact _output_get)))