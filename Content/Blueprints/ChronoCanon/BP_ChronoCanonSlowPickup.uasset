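; BP_ChronoCanonSlowPickup is a world pickup that gives the first-person player the ChronoCanon weapon, with its mesh spinning every tick.
; When the player overlaps the sphere, it calls AddBPChronoCanon on the character and snaps the mesh to the arms' GripPoint socket.
; It then destroys itself, plays a 2D pickup sound and shows the Widget_RamasserGun pickup widget.
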(event OnComponentBeginOverlap(Sphere)
  (params (OverlappedComponent :type Primitive%20Component%20Object%20Reference) (OtherActor :type Actor%20Object%20Reference) (OtherComp :type Primitive%20Component%20Object%20Reference) (OtherBodyIndex :type Integer) (bFromSweep :type Boolean) (SweepResult :type Hit%20Result%20Structure%20%28by%20ref%29))
  (bind _asbp_first_person_character (Utilities|Casting|CastToBP_FirstPersonCharacter OtherActor))
  (bind _output_get (Variables|Default|SetPlayer _asbp_first_person_character))
  (AddComponent|AddBPChronoCanon _output_get false)
  (Transformation|AttachComponentToComponent (Variables|Default|GetChronoCanonMesh) (Variables|/Game/FirstPerson/Blueprints/BP_FirstPersonCharacter.BP_FirstPersonCharacter_C|GetFirstPersonMesh _output_get) "GripPoint" "SnapToTarget" "SnapToTarget" "SnapToTarget" true)
  (Actor|DestroyActor)
  (Audio|PlaySound2D "/Game/Sounds/Interaction/Ramasser_fusil.Ramasser_fusil" 1.0 1.0 0.0 0 0)
  (bind _returnvalue (UserInterface|CreateWidget "/Game/UI/Tutoriels/Widget_RamasserGun.Widget_RamasserGun_C"))
  (UserInterface|Viewport|AddtoViewport _returnvalue 0))

(event EventTick
  (params (DeltaSeconds :type Float%20%28single-precision%29))
  (Transformation|AddLocalRotation (Variables|Default|GetChronoCanonMesh) "0.000000,1.000000,0.000000" false false))

(fn ConstructionScript)