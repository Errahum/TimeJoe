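; Pickup for the ChronoCanon speed ("Fast") module that floats in the level until the player collects it.
; Sphere overlap by BP_FirstPersonCharacter sets HasSpeed on the character, destroys the pickup and adds the Widget_RamasserFast prompt to the viewport.
; Tick spins the Cube by a fixed step per frame, while a ping-pong Timeline scaled by Height drives its up-and-down bob.
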(event OnComponentBeginOverlap(Sphere)
  (params (OverlappedComponent :type Primitive%20Component%20Object%20Reference) (OtherActor :type Actor%20Object%20Reference) (OtherComp :type Primitive%20Component%20Object%20Reference) (OtherBodyIndex :type Integer) (bFromSweep :type Boolean) (SweepResult :type Hit%20Result%20Structure%20%28by%20ref%29))
  ;[1 1 1] Affiche l'indication de prendre le module
  (bind _asbp_first_person_character (Utilities|Casting|CastToBP_FirstPersonCharacter OtherActor))
  (Variables|/Game/FirstPerson/Blueprints/BP_FirstPersonCharacter.BP_FirstPersonCharacter_C|SetHasSpeed _asbp_first_person_character true)
  (Actor|DestroyActor)
  (bind _returnvalue (UserInterface|CreateWidget "/Game/UI/Tutoriels/Widget_RamasserFast.Widget_RamasserFast_C"))
  (UserInterface|Viewport|AddtoViewport _returnvalue 0))

(event EventTick
  (params (DeltaSeconds :type Float%20%28single-precision%29))
  ;[1 1 1] Animation de rotation au model
  (Transformation|AddLocalRotation (Variables|Default|GetCube) "0.000000,1.000000,0.000000" false false))

(event EventBeginPlay
  ;[1 1 1] Ajoute l'animation du mouvement up down
  (bind _newtrack_0 (Timeline|Timeline Play)
    (:Update
      (Transformation|SetRelativeLocation (Variables|Default|GetCube) (Math|Vector|MakeVector 0.0 0.0 (* (Variables|Default|GetHeight) _newtrack_0)) false false))
    (:Finished
      (if (Variables|Default|GetIsReversing)
        (Variables|Default|SetIsReversing false)
        (Timeline|Timeline Play)
        (else
          (Variables|Default|SetIsReversing true)
          (Timeline|Timeline ReverseFromEnd))))))

(fn ConstructionScript)