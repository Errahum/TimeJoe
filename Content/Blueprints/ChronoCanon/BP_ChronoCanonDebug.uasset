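; Debug-instrumented ChronoCanon, a first-person weapon attached to the player that fires slow, fast or stop time zones.
; A camera trace spawns or replaces zones after a distance-based delay, attaching them to hit components so they follow moving objects.
; Zone and parent arrays support replacement, deletion with charge refund, and recycling the first zone when charges run out.
; Modules enable type switching; Tick prints state, updates the weapon material and disables it while grabbing.
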(event Input|EnhancedActionEvents|EnhancedInputActionIA_ModuleAttach
  (params (ActionValue :type Boolean) (ElapsedSeconds :type Float%20%28double-precision%29) (TriggeredSeconds :type Float%20%28double-precision%29) (InputAction :type Input%20Action%20Object%20Reference :default "/Game/FirstPerson/Input/Actions/IA_ModuleAttach.IA_ModuleAttach"))
  (bind _player (Variables|Default|GetPlayer))
  (bind _firstpersoncamera (Variables|/Game/FirstPerson/Blueprints/BP_FirstPersonCharacter.BP_FirstPersonCharacter_C|GetFirstPersonCamera _player))
  (bind _returnvalue (Transformation|GetWorldLocation _firstpersoncamera))
  (:Triggered
    (if (Variables|Default|GetIsGrabbing)
      (Development|PrintString "Tenir le ChronoCanon")
      (else
        (bind _outactors (Actor|GetAllActorsOfClass "/Game/Blueprints/Zones/BP_ZoneTemps.BP_ZoneTemps_C"))
        (bind _outhit (Collision|LineTraceByChannel _returnvalue (+ _returnvalue (* (Math|Vector|GetForwardVector (Transformation|GetWorldRotation _firstpersoncamera)) 2e+02)) "TraceTypeQuery1" false _outactors "None"))
        (if (Actor|ActorHasTag (.HitActor (Collision|BreakHitResult _outhit)) "Module")
          (if (Actor|ActorHasTag (.HitActor (Collision|BreakHitResult _outhit)) "zFast")
            (Variables|Default|SetFastActive? true)
            (elif (Actor|ActorHasTag (.HitActor (Collision|BreakHitResult _outhit)) "zStop")
              (Variables|Default|SetStopActive? true)))
          (else
            (Development|PrintString "Pas un module")))))))

(event Input|EnhancedActionEvents|EnhancedInputActionIA_Shoot
  (params (ActionValue :type Boolean) (ElapsedSeconds :type Float%20%28double-precision%29) (TriggeredSeconds :type Float%20%28double-precision%29) (InputAction :type Input%20Action%20Object%20Reference :default "/Game/FirstPerson/Input/Actions/IA_Shoot.IA_Shoot"))
  (bind _player (Variables|Default|GetPlayer))
  (bind _firstpersoncamera (Variables|/Game/FirstPerson/Blueprints/BP_FirstPersonCharacter.BP_FirstPersonCharacter_C|GetFirstPersonCamera _player))
  (bind _returnvalue (Transformation|GetWorldLocation _firstpersoncamera))
  (:Triggered
    (bind _outhit (CallFunction|Fire _returnvalue (+ _returnvalue (* (Math|Vector|GetForwardVector (Transformation|GetWorldRotation _firstpersoncamera)) (Variables|Default|GetMaxDistance)))))
    (Variables|Default|SetHitLocation (.Location (Collision|BreakHitResult _outhit)))
    (Animation|Montage|MontagePlay (Components|SkeletalMesh|GetAnimInstance (Variables|/Game/FirstPerson/Blueprints/BP_FirstPersonCharacter.BP_FirstPersonCharacter_C|GetFirstPersonMesh (Variables|Default|GetPlayer))) "/Game/FirstPersonArms/Animations/FP_Rifle_Shoot_Montage.FP_Rifle_Shoot_Montage" 1.0 "MontageLength" 0.0 false)
    (Variables|Default|SetHitComponent (.HitComponent (Collision|BreakHitResult _outhit)))
    (bind _output_get (Variables|Default|SetHit%20Actor (.HitActor (Collision|BreakHitResult _outhit))))
    (Utilities|IsValid _output_get
      (:Is%20Valid
        ;[1 1 1] Vérifie si le hit actor a les tags Untargetable ou Zone
        (if (Actor|ActorHasTag _output_get "Untargetable")
          (Development|PrintString "Untargetable")
          (elif (Actor|ActorHasTag _output_get "Zone")
            (Utilities|FlowControl|Delay (/ (.Distance (Collision|BreakHitResult _outhit)) 7e+03))
            ;[1 1 1] Détermine quel type de zone à remplacer avec
            (switch int (Variables|Default|GetZoneType)
              (:0
                (CallFunction|ReplaceSlow (Math|Conversions|ToTransform(Vector) (Transformation|GetWorldLocation (.HitComponent (Collision|BreakHitResult _outhit))))))
              (:1
                (CallFunction|ReplaceFast (Math|Conversions|ToTransform(Vector) (Transformation|GetWorldLocation (.HitComponent (Collision|BreakHitResult _outhit))))))
              (:2
                (CallFunction|ReplaceStop (Math|Conversions|ToTransform(Vector) (Transformation|GetWorldLocation (.HitComponent (Collision|BreakHitResult _outhit)))))))
            (Utilities|FlowControl|Delay 0.2)
            (Variables|Default|SetIsDelay false)
            (else
              ;[1 1 1] Vérifie si le joueur n'a plus de charges, si oui joue la fonction correspondante
              (if (Variables|Default|GetIsOutOfCharges)
                (CallFunction|OutOfCharges))
              (Utilities|FlowControl|Delay (/ (.Distance (Collision|BreakHitResult _outhit)) 7e+03))
              ;[1 1 1] Détermine quel type de zone a spawner.
              (switch int (Variables|Default|GetZoneType)
                (:0
                  (CallFunction|SpawnSlow (Math|Conversions|ToTransform(Vector) (.Location (Collision|BreakHitResult _outhit)))))
                (:1
                  (CallFunction|SpawnFast (Math|Conversions|ToTransform(Vector) (.Location (Collision|BreakHitResult _outhit)))))
                (:2
                  (CallFunction|SpawnStop (Math|Conversions|ToTransform(Vector) (.Location (Collision|BreakHitResult _outhit))))))
              (Utilities|FlowControl|Delay 0.2)
              (Variables|Default|SetIsDelay false))))))))

(event Input|EnhancedActionEvents|EnhancedInputActionIA_ZoneDelete
  (params (ActionValue :type Boolean) (ElapsedSeconds :type Float%20%28double-precision%29) (TriggeredSeconds :type Float%20%28double-precision%29) (InputAction :type Input%20Action%20Object%20Reference :default "/Game/FirstPerson/Input/Actions/IA_ZoneDelete.IA_ZoneDelete"))
  (bind _zonesarray (Variables|Default|GetZonesArray))
  (bind _parentarray (Variables|Default|GetParentArray))
  (bind _player (Variables|Default|GetPlayer))
  (bind _firstpersoncamera (Variables|/Game/FirstPerson/Blueprints/BP_FirstPersonCharacter.BP_FirstPersonCharacter_C|GetFirstPersonCamera _player))
  (bind _returnvalue (Transformation|GetWorldLocation _firstpersoncamera))
  (:Triggered
    (if (not (Variables|Default|GetIsGrabbing))
      (if (not (Variables|Default|GetIsShooting))
        (bind _outhit (Collision|LineTraceByChannel _returnvalue (+ _returnvalue (* (Math|Vector|GetForwardVector (Transformation|GetWorldRotation _firstpersoncamera)) (Variables|Default|GetMaxDistance))) "TraceTypeQuery3" false (Utilities|Array|MakeArray (Variables|Default|GetBP_Vitre)) "ForDuration"))
        (if (Actor|ActorHasTag (.HitActor (Collision|BreakHitResult _outhit)) "Zone")
          (bind _output_get (Variables|Default|SetIndexReplace (Utilities|Array|FindItem _zonesarray (.HitActor (Collision|BreakHitResult _outhit)))))
          (Utilities|Array|RemoveItem _parentarray (Utilities|Array|Get(acopy) _parentarray _output_get))
          (Utilities|Array|RemoveItem _zonesarray (.HitActor (Collision|BreakHitResult _outhit)))
          (Actor|DestroyActor (.HitActor (Collision|BreakHitResult _outhit)))
          (Variables|Default|SetCharges (+ (Variables|Default|GetCharges) 1))
          (else
            (Development|PrintString "WHAT DUH HELL")))))))

(event Input|EnhancedActionEvents|EnhancedInputActionIA_ZoneSlow
  (params (ActionValue :type Boolean) (ElapsedSeconds :type Float%20%28double-precision%29) (TriggeredSeconds :type Float%20%28double-precision%29) (InputAction :type Input%20Action%20Object%20Reference :default "/Game/FirstPerson/Input/Actions/IA_ZoneSlow.IA_ZoneSlow"))
  (:Triggered
    (if (not (Variables|Default|GetIsGrabbing))
      (Variables|Default|SetZoneType 0))))

(event Input|EnhancedActionEvents|EnhancedInputActionIA_ZoneAccelere
  (params (ActionValue :type Boolean) (ElapsedSeconds :type Float%20%28double-precision%29) (TriggeredSeconds :type Float%20%28double-precision%29) (InputAction :type Input%20Action%20Object%20Reference :default "/Game/FirstPerson/Input/Actions/IA_ZoneAccelere.IA_ZoneAccelere"))
  (:Triggered
    (if (not (Variables|Default|GetIsGrabbing))
      (if (Variables|Default|GetStopActive?)
        (Variables|Default|SetZoneType 2)))))

(event Input|EnhancedActionEvents|EnhancedInputActionIA_ZoneStop
  (params (ActionValue :type Boolean) (ElapsedSeconds :type Float%20%28double-precision%29) (TriggeredSeconds :type Float%20%28double-precision%29) (InputAction :type Input%20Action%20Object%20Reference :default "/Game/FirstPerson/Input/Actions/IA_ZoneStop.IA_ZoneStop"))
  (:Triggered
    (if (not (Variables|Default|GetIsGrabbing))
      (if (Variables|Default|GetFastActive?)
        (Variables|Default|SetZoneType 1)))))

(event Input|EnhancedActionEvents|EnhancedInputActionIA_ChangementScrollUp
  (params (ActionValue :type Boolean) (ElapsedSeconds :type Float%20%28double-precision%29) (TriggeredSeconds :type Float%20%28double-precision%29) (InputAction :type Input%20Action%20Object%20Reference :default "/Game/FirstPerson/Input/Actions/IA_ChangementScrollUp.IA_ChangementScrollUp"))
  (:Triggered
    (if (not (Variables|Default|GetIsGrabbing))
      (if (Variables|Default|GetStopActive?)
        (if (Variables|Default|GetFastActive?)
          (if (== (Variables|Default|GetZoneType) 2)
            (Variables|Default|SetZoneType 0)
            (else
              (Variables|Default|SetZoneType (+ (Variables|Default|GetZoneType) 1))))
          (elif (== (Variables|Default|GetZoneType) 1)
            (Variables|Default|SetZoneType 0)
            (else
              (Variables|Default|SetZoneType (+ (Variables|Default|GetZoneType) 1)))))
        (else
          (Development|PrintString "Module Missing"))))))

(event Input|EnhancedActionEvents|EnhancedInputActionIA_ChangementScrollDown
  (params (ActionValue :type Boolean) (ElapsedSeconds :type Float%20%28double-precision%29) (TriggeredSeconds :type Float%20%28double-precision%29) (InputAction :type Input%20Action%20Object%20Reference :default "/Game/FirstPerson/Input/Actions/IA_ChangementScrollDown.IA_ChangementScrollDown"))
  (:Triggered
    (if (not (Variables|Default|GetIsGrabbing))
      (if (Variables|Default|GetStopActive?)
        (if (Variables|Default|GetFastActive?)
          (if (== (Variables|Default|GetZoneType) 0)
            (Variables|Default|SetZoneType 2)
            (else
              (Variables|Default|SetZoneType (- (Variables|Default|GetZoneType) 1))))
          (elif (== (Variables|Default|GetZoneType) 0)
            (Variables|Default|SetZoneType 1)
            (else
              (Variables|Default|SetZoneType (- (Variables|Default|GetZoneType) 1)))))
        (else
          (Development|PrintString "Module Missing"))))))

(event EventBeginPlay
  (bind _player (Variables|Default|GetPlayer))
  (Development|PrintString "Attached")
  (CallFunction|AttachWeapon)
  ;[1 1 1] Ajoute les contrôles du ChronoCanon au joueur et set l'animation du ChronoCanon
  (Variables|/Game/FirstPerson/Blueprints/BP_FirstPersonCharacter.BP_FirstPersonCharacter_C|SetbHasRifle _player true)
  (bind _asplayer_controller (Utilities|Casting|CastToPlayerController (Pawn|GetController _player)))
  (Utilities|IsValid (PlayerController|LocalPlayerSubsystems|GetEnhancedInputLocalPlayerSubsystem _asplayer_controller)
    (:Is%20Valid
      (Input|AddMappingContext (PlayerController|LocalPlayerSubsystems|GetEnhancedInputLocalPlayerSubsystem _asplayer_controller) "/Game/FirstPerson/Input/IMC_Weapons.IMC_Weapons" 0 "(bIgnoreAllPressedKeysUntilRelease=True,bForceImmediately=False)"))))

(event EventTick
  (params (DeltaSeconds :type Float%20%28single-precision%29))
  (bind _player (Variables|Default|GetPlayer))
  (CallFunction|VerificationCube)
  (Development|PrintString (Utilities|String|Append "Type : " (Utilities|String|ToString(Integer) (Variables|Default|GetZoneType)) " 
Charges : " (Utilities|String|ToString(Integer) (Variables|Default|GetCharges)) " 
Nombre de Zones : " (Utilities|String|ToString(Integer) (Utilities|Array|Length (Variables|Default|GetZonesArray))) " 
IndexNumber : " (Utilities|String|ToString(Integer) (Variables|Default|GetIndexNumber)) " 
Out of charges : " (Utilities|String|ToString(Boolean) (Variables|Default|GetIsOutOfCharges)) (Variables|Default|GetAttachedObject) " 
Stop Attached? :" (Utilities|String|ToString(Boolean) (Variables|Default|GetStopActive?)) " 
Fast Attached? : " (Utilities|String|ToString(Boolean) (Variables|Default|GetFastActive?)) " 
IndexReplace : " (Utilities|String|ToString(Integer) (Variables|Default|GetIndexReplace))) true true "(R=0.000000,G=0.660000,B=1.000000,A=1.000000)" 0.0)
  (CallFunction|CalculeCharge)
  (CallFunction|ChangementDeCouleur)
  (if (Variables|/Game/FirstPerson/Blueprints/BP_FirstPersonCharacter.BP_FirstPersonCharacter_C|GetHasStop _player)
    (Variables|Default|SetStopActive? true))
  (if (Variables|/Game/FirstPerson/Blueprints/BP_FirstPersonCharacter.BP_FirstPersonCharacter_C|GetHasSpeed _player)
    (Variables|Default|SetFastActive? true)))

(fn CalculeCharge
  ;[1 1 1] Détermine si il reste 0 charges au joueur
  (if (== (Variables|Default|GetCharges) 0)
    (Variables|Default|SetIsOutOfCharges true)
    (else
      (Variables|Default|SetIsOutOfCharges false))))

(fn SpawnStop
  (params (SpawnTransform :type Transform))
  (bind _hitcomponent (Variables|Default|GetHitComponent))
  (bind _returnvalue (Game|SpawnActorfromClass "/Game/Blueprints/Zones/BP_ZoneTemps_Stop.BP_ZoneTemps_Stop_C" SpawnTransform "Undefined" (Variables|Default|GetHit%20Actor) (Variables|Default|GetPlayer)))
  (Transformation|AttachComponentToComponent _returnvalue _hitcomponent "None" "KeepWorld" "KeepWorld" "KeepWorld" true)
  (Utilities|Array|Add (Variables|Default|GetZonesArray) _returnvalue)
  (Utilities|Array|Add (Variables|Default|GetParentArray) _hitcomponent)
  (Variables|Default|SetCharges (- (Variables|Default|GetCharges) 1))
  (Variables|Default|SetIsShooting false)
  (Variables|Default|SetIsDelay true))

(fn SpawnFast
  (params (SpawnTransform :type Transform))
  (bind _hitcomponent (Variables|Default|GetHitComponent))
  (bind _returnvalue (Game|SpawnActorfromClass "/Game/Blueprints/Zones/BP_ZoneTemps_Fast.BP_ZoneTemps_Fast_C" SpawnTransform "Undefined" 0 (Variables|Default|GetPlayer)))
  (Transformation|AttachComponentToComponent _returnvalue _hitcomponent "None" "KeepWorld" "KeepWorld" "KeepWorld" true)
  (Utilities|Array|Add (Variables|Default|GetZonesArray) _returnvalue)
  (Utilities|Array|Add (Variables|Default|GetParentArray) _hitcomponent)
  (Variables|Default|SetCharges (- (Variables|Default|GetCharges) 1))
  (Variables|Default|SetIsShooting false)
  (Variables|Default|SetIsDelay true))

(fn SpawnSlow
  (params (SpawnTransform :type Transform))
  (bind _hitcomponent (Variables|Default|GetHitComponent))
  ;[1 1 1] Spawn la zone et l'attache au component qu'il a hit pour que la zone puisse bouger avec ex: piston et plateforme.
  (bind _returnvalue (Game|SpawnActorfromClass "/Game/Blueprints/Zones/BP_ZoneTemps_Slow.BP_ZoneTemps_Slow_C" SpawnTransform "Undefined" (Variables|Default|GetHit%20Actor) (Variables|Default|GetPlayer)))
  (Transformation|AttachComponentToComponent _returnvalue _hitcomponent "None" "KeepWorld" "KeepWorld" "KeepWorld" true)
  ;[1 1 1] Ajoute la zone dans la zone array et ajoute son parent dans un autre array, le
  (Utilities|Array|Add (Variables|Default|GetZonesArray) _returnvalue)
  (Utilities|Array|Add (Variables|Default|GetParentArray) _hitcomponent)
  (Variables|Default|SetCharges (- (Variables|Default|GetCharges) 1))
  (Variables|Default|SetIsShooting false)
  (Variables|Default|SetIsDelay true))

(fn ReplaceSlow
  (params (SpawnTransform :type Transform))
  (bind _hit_actor (Variables|Default|GetHit%20Actor))
  (bind _zonesarray (Variables|Default|GetZonesArray))
  (Variables|Default|SetIndexReplace (Utilities|Array|FindItem _zonesarray _hit_actor))
  (Utilities|Array|RemoveItem _zonesarray _hit_actor)
  (if (Actor|ActorHasTag _hit_actor "Zone")
    (Actor|DestroyActor _hit_actor)
    (Variables|Default|SetUsedParent 0)
    (bind _returnvalue (Game|SpawnActorfromClass "/Game/Blueprints/Zones/BP_ZoneTemps_Slow.BP_ZoneTemps_Slow_C" SpawnTransform "Undefined" 0 (Variables|Default|GetPlayer)))
    (Transformation|AttachComponentToComponent _returnvalue (Utilities|Array|Get(acopy) (Variables|Default|GetParentArray) (Variables|Default|GetIndexReplace)) "None" "KeepWorld" "KeepWorld" "KeepWorld" true)
    (Utilities|Array|Add (Variables|Default|GetZonesArray) _returnvalue)
    (Variables|Default|SetIsShooting false)
    (Variables|Default|SetIsDelay true)))

(fn ReplaceFast
  (params (SpawnTransform :type Transform))
  (bind _hit_actor (Variables|Default|GetHit%20Actor))
  (bind _zonesarray (Variables|Default|GetZonesArray))
  (Variables|Default|SetIndexReplace (Utilities|Array|FindItem _zonesarray _hit_actor))
  (Utilities|Array|RemoveItem _zonesarray _hit_actor)
  (if (Actor|ActorHasTag _hit_actor "Zone")
    (Actor|DestroyActor _hit_actor)
    (bind _returnvalue (Game|SpawnActorfromClass "/Game/Blueprints/Zones/BP_ZoneTemps_Fast.BP_ZoneTemps_Fast_C" SpawnTransform "Undefined" 0 (Variables|Default|GetPlayer)))
    (Transformation|AttachComponentToComponent _returnvalue (Utilities|Array|Get(acopy) (Variables|Default|GetParentArray) (Variables|Default|GetIndexReplace)) "None" "KeepWorld" "KeepWorld" "KeepWorld" true)
    (Utilities|Array|Add (Variables|Default|GetZonesArray) _returnvalue)
    (Variables|Default|SetIsShooting false)
    (Variables|Default|SetIsDelay true)))

(fn ReplaceStop
  (params (SpawnTransform :type Transform))
  (bind _hit_actor (Variables|Default|GetHit%20Actor))
  (bind _zonesarray (Variables|Default|GetZonesArray))
  (Variables|Default|SetIndexReplace (Utilities|Array|FindItem _zonesarray _hit_actor))
  (Utilities|Array|RemoveItem _zonesarray _hit_actor)
  (if (Actor|ActorHasTag _hit_actor "Zone")
    (Actor|DestroyActor _hit_actor)
    (bind _returnvalue (Game|SpawnActorfromClass "/Game/Blueprints/Zones/BP_ZoneTemps_Stop.BP_ZoneTemps_Stop_C" SpawnTransform "Undefined" (Variables|Default|GetHit%20Actor) (Variables|Default|GetPlayer)))
    (Transformation|AttachComponentToComponent _returnvalue (Utilities|Array|Get(acopy) (Variables|Default|GetParentArray) (Variables|Default|GetIndexReplace)) "None" "KeepWorld" "KeepWorld" "KeepWorld" true)
    (Utilities|Array|Add (Variables|Default|GetZonesArray) _returnvalue)
    (Variables|Default|SetIsShooting false)
    (Variables|Default|SetIsDelay true)))

(fn OutOfCharges
  (bind _zonesarray (Variables|Default|GetZonesArray))
  ;[1 1 1] Identifie la zone la plus ancienne et l'enlève du array et le destroy, ensuite ajoute une charge au joueur.
  (Actor|DestroyActor (Utilities|Array|Get(acopy) _zonesarray (Variables|Default|GetIndexNumber)))
  (Utilities|Array|RemoveItem _zonesarray (Utilities|Array|Get(acopy) _zonesarray (Variables|Default|GetIndexNumber)))
  (Variables|Default|SetIndexNumber 0)
  (Variables|Default|SetCharges 1))

(fn ChangementDeCouleur
  ;[1 1 1] Change la texture du ChronoCanon selon le type de zone.
  (switch int (Variables|Default|GetZoneType)
    (:0
      (Rendering|Material|SetMaterial 0 "/Game/Assets/ChronoCanon/M_ChronoCanon.M_ChronoCanon"))
    (:1
      (Rendering|Material|SetMaterial 0 "/Game/Assets/ChronoCanon/M_ChronoCanon_3.M_ChronoCanon_3"))
    (:2
      (Rendering|Material|SetMaterial 0 "/Game/Assets/ChronoCanon/M_ChronoCanon_22.M_ChronoCanon_22"))))

(fn VerificationCube
  (bind _player (Variables|Default|GetPlayer))
  ;[1 1 1] Verifie si le joueur prend un cube, et désactive le ChronoCanon au besoin.
  (if (Variables|/Game/FirstPerson/Blueprints/BP_FirstPersonCharacter.BP_FirstPersonCharacter_C|GetIsGrabbing _player)
    (Variables|/Game/FirstPerson/Blueprints/BP_FirstPersonCharacter.BP_FirstPersonCharacter_C|SetbHasRifle _player false)
    (Variables|Default|SetIsGrabbing true)
    (else
      (Variables|Default|SetIsGrabbing false)
      (Variables|/Game/FirstPerson/Blueprints/BP_FirstPersonCharacter.BP_FirstPersonCharacter_C|SetbHasRifle _player true))))

(fn AttachWeapon
  ;[1 1 1] Attache le ChronoCanon à la main du joueur
  (bind _asbp_first_person_character (Utilities|Casting|CastToBP_FirstPersonCharacter (Components|GetOwner)))
  (bind _output_get (Variables|Default|SetPlayer _asbp_first_person_character))
  (Transformation|AttachComponentToComponent (Variables|/Game/FirstPerson/Blueprints/BP_FirstPersonCharacter.BP_FirstPersonCharacter_C|GetFirstPersonMesh _output_get) "GripPoint" "SnapToTarget" "SnapToTarget" "SnapToTarget" true))

(fn Fire
  (params (LineStart :type Vector) (LineEnd :type Vector))
  ;[1 1 1] Verifie que les conditions sont respectées, et tire un line trace.
  (if (not (Variables|Default|GetIsGrabbing))
    (if (Variables|Default|GetIsDelay)
      _
      (else
        (Variables|Default|SetIsShooting true)
        (bind _outhit (Collision|LineTraceByChannel LineStart LineEnd "TraceTypeQuery2" false 0 "ForDuration"))))
    (return 0 _outhit)))

(fn PlayAnim
  (params (Hit%20Actor :type Actor%20Object%20Reference) (HitComponent :type Primitive%20Component%20Object%20Reference) (self2 :type BP%20First%20Person%20Character%20Object%20Reference) (InputPin :type Vector))
  ;[1 1 1] Joue l'animation de tire, et set des variables du hit result provenant du line trace
  (Variables|Default|SetHitLocation InputPin)
  (Animation|Montage|MontagePlay (Components|SkeletalMesh|GetAnimInstance (Variables|/Game/FirstPerson/Blueprints/BP_FirstPersonCharacter.BP_FirstPersonCharacter_C|GetFirstPersonMesh self2)) "/Game/FirstPersonArms/Animations/FP_Rifle_Shoot_Montage.FP_Rifle_Shoot_Montage" 1.0 "MontageLength" 0.0 false)
  (Variables|Default|SetHitComponent HitComponent)
  (return 0))