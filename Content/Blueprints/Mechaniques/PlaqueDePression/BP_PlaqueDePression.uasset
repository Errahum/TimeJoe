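; BP_PlaqueDePression is a pressure plate that activates and deactivates the actors in its ActivationList.
; Any overlapping actor not tagged "Zone" sends ActivateMessage through BPI_Activate, while Deactivate waits until the Box is empty.
; Each successful interface cast also plays the press or reset sound and moves the Plaque mesh down or up, so this feedback runs inside the loop.
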(event EventBeginPlay)

(event Collision|EventActorBeginOverlap
  (params (OtherActor :type Actor%20Object%20Reference))
  ;[0 1 0.6535] Condition pour savoir s'il y a une tags "zone". Le projectile de zone ne doit pas activer la plaque de pression.
  (if (not (Actor|ActorHasTag OtherActor "Zone"))
    (Development|PrintString "Plaque De Pression Activate")
    ;[0 1 0.7757] Tous les objets du tableau seront activés et désactivés.
    (for _array_element (Variables|Default|GetActivationList)
      (bind _asbpi_activate (Utilities|Casting|CastToBPI_Activate _array_element))
      ;[0 0.06341 1] Active l'interface d'activation pour les objets affecté
      (Class|BPIActivate|Activate(Message) (Utilities|ToObject(Interface) _asbpi_activate))
      ;[0 1 0.5095] Le son d'activation et de désactivation du bouton.
      (Audio|PlaySoundatLocation "/Game/Sounds/Interaction/Pressure_Plate/Pressure_Press.Pressure_Press" (Transformation|GetActorLocation) "0, 0, 0" 1.0 1.0 0.0 0 0 0 0)
      ;[0 0.25 1] Une animation pour l'activation.
      (CallFunction|AnimationActivation))))

(event EventTick
  (params (DeltaSeconds :type Float%20%28single-precision%29)))

(event Collision|EventActorEndOverlap
  (params (OtherActor :type Actor%20Object%20Reference))
  ;[0 1 0.6535] Condition pour savoir s'il y a une tags "zone". Le projectile de zone ne doit pas activer la plaque de pression.
  (if (not (or (Actor|ActorHasTag OtherActor "Zone") (Utilities|Array|IsNotEmpty (Collision|GetOverlappingActors (Variables|Default|GetBox) 0 :!class /Script/Engine.PrimitiveComponent))))
    (Development|PrintString "Plaque De Pression Deactivate")
    ;[0 1 0.7757] Tous les objets du tableau seront activés et désactivés.
    (for _array_element (Variables|Default|GetActivationList)
      (bind _asbpi_activate (Utilities|Casting|CastToBPI_Activate _array_element))
      ;[1 0 0.03784] Active l'interface de désactivation pour les objets affecté
      (Default|Deactivate _asbpi_activate)
      ;[0 1 0.5095] Le son d'activation et de désactivation du bouton.
      (Audio|PlaySoundatLocation "/Game/Sounds/Interaction/Pressure_Plate/Pressure_Reset.Pressure_Reset" (Transformation|GetActorLocation) "0, 0, 0" 1.0 1.0 0.0 0 0 0 0)
      ;[0.641 1 0] Une animation pour la désactivation.
      (CallFunction|AnimationDesactivation))))

(fn ConstructionScript)

(fn Activate
  (params (NewParam1 :type Boolean))
  (return false))

(fn AnimationActivation
  (Transformation|SetRelativeLocation (Variables|Default|GetPlaque) (Math|Vector|MakeVector 0.0 0.0 0.0) false false))

(fn AnimationDesactivation
  (Transformation|SetRelativeLocation (Variables|Default|GetPlaque) (Math|Vector|MakeVector 0.0 0.0 5.0) false false))