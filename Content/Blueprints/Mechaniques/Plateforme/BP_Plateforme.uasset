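; BP_Plateforme is a moving platform that shuttles back and forth between its actor origin and a MoveLocation component.
; BeginPlay scales the timeline's play rate by the travel distance, so PlayRate acts like a speed, then starts it after StartDelay.
; The timeline track multiplies MoveLocation's relative position to place the Plateforme component, without sweeping.
; On finish, the IsReversing flag alternates Play and Reverse for an endless ping-pong.
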(event EventBeginPlay
  (bind _movelocation (Variables|Default|GetMoveLocation))
  (bind _relativelocation (Variables|/Script/Engine.SceneComponent|GetRelativeLocation _movelocation))
  (Components|Timeline|SetPlayRate (Variables|Default|GetTimeline) (/ (Variables|Default|GetPlay%20Rate) (/ (Math|Vector|VectorLength (- (Variables|/Script/Engine.SceneComponent|GetRelativeLocation (Variables|Default|GetPlateforme)) _relativelocation)) 5e+02)))
  (Utilities|FlowControl|Delay (Variables|Default|GetStartDelay))
  (bind _newtrack_0 (Timeline|Timeline Play)
    (:Update
      (Transformation|SetRelativeLocation (Variables|Default|GetPlateforme) (* _newtrack_0 _relativelocation) false false))
    (:Finished
      (if (Variables|Default|GetIsReversing)
        (Variables|Default|SetIsReversing false)
        (Timeline|Timeline Play)
        (else
          (Variables|Default|SetIsReversing true)
          (Timeline|Timeline Reverse))))))

(fn ConstructionScript)