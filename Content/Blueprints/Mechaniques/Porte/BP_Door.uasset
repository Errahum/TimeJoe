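; BP_Door is an activatable double sliding door that responds to Activate and Deactivate with sound and animation.
; A timeline alpha drives OuverturePorte, which moves the left and right panels to opposite Y offsets scaled by DoorOpenDistance.
; StartOpen places the panels open at construction and switches activation to a separate inversion timeline with swapped sounds.
; Deactivate reverses the active timeline, and GetDeactivationTime exposes the button deactivation delay.
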(event Custom|Door_Inverse_Start
  ;[0 1 0.6263] L'event qui sert à ouvrir la porte à l'inverse.
  (CallFunction|PorteOuverteInversion))

(event EventActivate
  (bind _returnvalue (Transformation|GetActorLocation))
  ;[0 1 0.4871] Condition Pour savoir si la porte à le Bool "PorteOuvreInverse"
  (if (Variables|Default|GetPorteOuvreInverse)
    ;[0 1 0.4087] Le son de la porte quand il s'ouvre et il se ferme.
    (Audio|PlaySoundatLocation "/Game/Sounds/Door/Door_Open.Door_Open" _returnvalue "0, 0, 0" 1.0 1.0 0.0 0 0 0 0)
    (Variables|Default|SetIs_Active true)
    ;[0 0.2762 1] Timeline qui est pour une ouverture et une fermeture de la porte.
    (bind _alpha (Timeline|Timeline_Normal Play)
      (:Update
        (CallFunction|OuverturePorte _alpha)))
    (else
      (Audio|PlaySoundatLocation "/Game/Sounds/Door/Door_Close.Door_Close" _returnvalue "0, 0, 0" 1.0 1.0 0.0 0 0 0 0)
      (Variables|Default|SetIs_Active true)
      (bind _alpha_2 (Timeline|Timeline_Inversion Play)
        (:Update
          (CallFunction|OuverturePorte _alpha_2))))))

(event EventDeactivate
  (bind _returnvalue (Transformation|GetActorLocation))
  ;[0 1 0.4871] Condition Pour savoir si la porte à le Bool "PorteOuvreInverse"
  (if (Variables|Default|GetPorteOuvreInverse)
    ;[0 1 0.4087] Le son de la porte quand il s'ouvre et il se ferme.
    (Audio|PlaySoundatLocation "/Game/Sounds/Door/Door_Close.Door_Close" _returnvalue "0, 0, 0" 1.0 1.0 0.0 0 0 0 0)
    (Variables|Default|SetIs_Active false)
    ;[0 0.2762 1] Timeline qui est pour une ouverture et une fermeture de la porte.
    (bind _alpha (Timeline|Timeline_Normal Reverse)
      (:Update
        (CallFunction|OuverturePorte _alpha)))
    (else
      (Audio|PlaySoundatLocation "/Game/Sounds/Door/Door_Open.Door_Open" _returnvalue "0, 0, 0" 1.0 1.0 0.0 0 0 0 0)
      (Variables|Default|SetIs_Active false)
      (bind _alpha_2 (Timeline|Timeline_Inversion Reverse)
        (:Update
          (CallFunction|OuverturePorte _alpha_2))))))

(fn ConstructionScript
  (Components|Timeline|SetPlayRate (Variables|Default|GetTimeline_Normal) 1.0)
  ;[0 1 0.5277] Si "StartOpen" est activé par le game designer, l'event "Door Inverse Start est appelé.
  (if (Variables|Default|GetStartOpen)
    (Variables|Default|SetPorteOuvreInverse false)
    (CallFunction|DoorInverseStart)
    (else
      (Variables|Default|SetPorteOuvreInverse true))))

(fn OuverturePorte
  (params (A :type Float%20%28double-precision%29))
  (bind _dooropendistance (Variables|Components|GetDoorOpenDistance))
  (bind _returnvalue (* A _dooropendistance))
  (Transformation|SetRelativeLocation (Variables|Default|GetPorteGauche) (Math|Vector|MakeVector 0.0 _returnvalue 0.0) false false)
  (Transformation|SetRelativeLocation (Variables|Default|GetPorteDroite) (Math|Vector|MakeVector 0.0 (* _returnvalue -1.0) 0.0) false false))

(fn PorteOuverteInversion
  (bind _dooropendistance (Variables|Components|GetDoorOpenDistance))
  (Transformation|SetRelativeLocation (Variables|Default|GetPorteGauche) (Math|Vector|MakeVector 0.0 _dooropendistance 0.0) false false)
  (Transformation|SetRelativeLocation (Variables|Default|GetPorteDroite) (Math|Vector|MakeVector 0.0 (* _dooropendistance -1.0) 0.0) false false))

(fn GetDeactivationTime
  (return (Variables|Default|GetBouton_Temps_Desactivation)))