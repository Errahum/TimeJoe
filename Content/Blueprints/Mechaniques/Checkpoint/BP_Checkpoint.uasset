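; Checkpoint actor that becomes the player's current checkpoint when the player overlaps it.
; On overlap, it checks the Player tag, casts to BP_FirstPersonCharacter, stores itself as CurrentCheckpoint and prints the new respawn name.
; A DoOnce then calls ResetZones on the BPReset reference, so zones reset only the first time the checkpoint is reached.
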(event EventBeginPlay)

(event Collision|EventActorBeginOverlap
  (params (OtherActor :type Actor%20Object%20Reference))
  (bind _self self)
  (if (Actor|ActorHasTag OtherActor "Player")
    (bind _asbp_first_person_character (Utilities|Casting|CastToBP_FirstPersonCharacter OtherActor))
    (Variables|/Game/FirstPerson/Blueprints/BP_FirstPersonCharacter.BP_FirstPersonCharacter_C|SetCurrentCheckpoint _asbp_first_person_character _self)
    (Development|PrintString (Utilities|String|Append "Respawn set to " (Utilities|GetDisplayName _self)))
    (Utilities|FlowControl|DoOnce false
      (:Completed
        (Default|ResetZones (Variables|Default|GetBP_Reset))))))

(event EventTick
  (params (DeltaSeconds :type Float%20%28single-precision%29)))

(fn ConstructionScript)