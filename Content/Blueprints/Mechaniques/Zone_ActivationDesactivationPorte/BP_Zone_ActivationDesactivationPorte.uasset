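; BP_Zone_ActivationDesactivationPorte is a trigger zone that activates or deactivates a BP_Door when an actor overlaps it.
; The first overlap passes a DoOnce, waits a configurable delay, then calls Activate on the door if DoorStartOpen is true, or Deactivate otherwise.
; An older loop over multiple doors using BPI_Activate remains in an unused graph, and the zone's own Activate function only returns false.
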(event EventBeginPlay)

(event Collision|EventActorBeginOverlap
  (params (OtherActor :type Actor%20Object%20Reference))
  (Utilities|FlowControl|DoOnce false
    (:Completed
      (Utilities|FlowControl|Delay (Variables|Default|GetDelay))
      (if (Variables|Default|GetDoorStartOpen)
        (Development|PrintString "Inversed")
        (bind _asbp_door (Utilities|Casting|CastToBP_Door (Variables|Default|GetActivationList)))
        (Default|Activate _asbp_door)
        (else
          (Development|PrintString "Inversed")
          (bind _asbp_door_2 (Utilities|Casting|CastToBP_Door (Variables|Default|GetActivationList)))
          (Default|Deactivate _asbp_door_2))))))

(event EventTick
  (params (DeltaSeconds :type Float%20%28single-precision%29)))

(fn ConstructionScript)

(fn Activate
  (params (NewParam1 :type Boolean))
  (return false))