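; BP_LaserFX_Place is a laser effect actor that draws a colored Niagara beam.
; Every tick it line traces on Visibility along its forward vector over a set length, then passes the LaserEnd variable and color to the beam.
; The trace result is not visibly used, and the impact effect's color and hit-position updates are disconnected.
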(event EventBeginPlay
  ;[1 0 0] La couleur du laser
  (Effects|Components|ParticleSystem|SetColorParameter (Variables|Default|GetNiagaraLaser) "Color" (Variables|Default|GetLaser_Color)))

(event EventTick
  (params (DeltaSeconds :type Float%20%28single-precision%29))
  (CallFunction|LineTraceLaser))

(fn ConstructionScript)

(fn LineTraceLaser
  (bind _returnvalue (Transformation|GetActorLocation))
  (bind _returnvalue_2 (Transformation|GetActorForwardVector))
  (bind _longueur_laser (Variables|Default|GetLongueur_Laser))
  (bind _returnvalue_3 (* _returnvalue_2 _longueur_laser))
  (bind _returnvalue_4 (+ _returnvalue _returnvalue_3))
  (Variables|Default|SetTraceEnd _returnvalue_4)
  (Collision|LineTraceByChannel _returnvalue _returnvalue_4 "TraceTypeQuery1" false 0 "None")
  ;[0 1 0.5415] Détermine ou que le laser s'arrête.
  (Effects|Components|ParticleSystem|SetVectorParameter (Variables|Default|GetNiagaraLaser) "LaserEnd" (Variables|Default|GetLaser_End))
  (Effects|Components|ParticleSystem|SetColorParameter (Variables|Default|GetNiagaraLaser) "Color" (Variables|Default|GetLaser_Color)))