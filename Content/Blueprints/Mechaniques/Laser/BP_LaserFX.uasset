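; Laser effect actor that builds a configurable set of colored Niagara beams, each stopping at whatever blocks it.
; Construction spawns the beams with stepped Y offset and roll.
; A visibility line trace from each Niagara child along actor forward, ignoring BP_ZoneTemps, sets LaserEnd to hit or maximum length, refreshed on Tick when enabled.
; Impact visibility is set only during construction; its repositioning logic is unconnected.
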(event EventBeginPlay
  ;[1 0 0] La couleur du laser
  (Effects|Components|ParticleSystem|SetColorParameter (Variables|Default|GetNiagaraLaser) "Color" (Variables|Default|GetLaser_Color))
  ;[0 0.1217 1] La couleur  de l'imact
  (Effects|Components|ParticleSystem|SetColorParameter (Variables|Default|GetNiagaraLaserImpact) "Color" "(R=0.028439,G=0.000000,B=1.000000,A=1.000000)"))

(event EventTick
  (params (DeltaSeconds :type Float%20%28single-precision%29))
  (if (Variables|Default|GetUpdate_LaserPosition)
    (CallFunction|LineTraceLaser)))

(fn ConstructionScript
  (for _index (range 0 (Variables|Default|GetNumLaser))
    (bind _returnvalue (AddComponent|AddNiagaraComponent false (Math|Transform|MakeTransform (Math|Vector|MakeVector 0.0 (Math|Conversions|ToFloat(Integer) (* _index 50)) 0.0) (Math|Rotator|MakeRotator (Math|Conversions|ToFloat(Integer) (* _index 50)) 0.0 0.0) "1.000000,1.000000,1.000000")))
    (Class|NiagaraComponent|SetAsset _returnvalue "/Game/VFX/Niagara/Laser/NS_Laser_System.NS_Laser_System" true)
    (Effects|Components|ParticleSystem|SetColorParameter _returnvalue "Color" (Variables|Default|GetLaser_Color))
    (Rendering|SetVisibility (Variables|Default|GetNiagaraLaserImpact) (Variables|Default|GetHit) false)
    (Transformation|AttachComponentToComponent _returnvalue (Variables|Default|GetDefaultSceneRoot) "None" "KeepRelative" "KeepRelative" "KeepRelative" true)
    (CallFunction|LineTraceLaser)))

(fn LineTraceLaser
  (for _array_element (Components|GetChildrenComponents (Variables|Default|GetDefaultSceneRoot) true)
    (bind _asniagara_particle_system_component (Utilities|Casting|CastToNiagaraComponent _array_element))
    (Variables|Default|SetAs%20Niagara%20Particle%20System%20Component _asniagara_particle_system_component)
    (Variables|Default|SetTraceEnd (+ (+ (Transformation|GetWorldLocation (Variables|Default|GetAs%20Niagara%20Particle%20System%20Component)) "0.000000,5.000000,0.000000") (* (Transformation|GetActorForwardVector) (Variables|Default|GetLongueur_Laser))))
    (bind _outactors (Actor|GetAllActorsOfClass "/Game/Blueprints/Zones/BP_ZoneTemps.BP_ZoneTemps_C"))
    (bind _outhit (Collision|LineTraceByChannel (+ (Transformation|GetWorldLocation (Variables|Default|GetAs%20Niagara%20Particle%20System%20Component)) "0.000000,5.000000,0.000000") (+ (+ (Transformation|GetWorldLocation (Variables|Default|GetAs%20Niagara%20Particle%20System%20Component)) "0.000000,5.000000,0.000000") (* (Transformation|GetActorForwardVector) (Variables|Default|GetLongueur_Laser))) "TraceTypeQuery1" false _outactors "None"))
    (Variables|Default|SetHit (.bblockinghit _outhit))
    (Variables|Default|SetHit_Location (.location _outhit))
    ;[0 1 0.5415] Détermine ou que le laser s'arrête.
    (Effects|Components|ParticleSystem|SetVectorParameter (Variables|Default|GetAs%20Niagara%20Particle%20System%20Component) "LaserEnd" (select (Variables|Default|GetHit) (Variables|Default|GetHit_Location) (Variables|Default|GetTraceEnd)))
    (Effects|Components|ParticleSystem|SetColorParameter (Variables|Default|GetNiagaraLaser) "Color" (Variables|Default|GetLaser_Color))))