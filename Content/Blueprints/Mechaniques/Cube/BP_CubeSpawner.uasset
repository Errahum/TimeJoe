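; BP_CubeSpawner is a cube dispenser actor that produces a BP_Cube below itself when activated.
; Activate plays the spawner sound and destroys the previously stored cube if still valid, so only one cube from this spawner exists at a time.
; It then spawns a new cube slightly beneath its own location and stores it as CubeInstance.
; GetDeactivationTime returns zero, and debug prints report the validity check.
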(event EventBeginPlay)

(event Collision|EventActorBeginOverlap
  (params (OtherActor :type Actor%20Object%20Reference)))

(event EventTick
  (params (DeltaSeconds :type Float%20%28single-precision%29)))

(event EventActivate
  (bind _returnvalue (Transformation|GetActorTransform))
  (Audio|PlaySoundatLocation "/Game/Sounds/Interaction/Spawner_Cube.Spawner_Cube" (Transformation|GetActorLocation) "0, 0, 0" 1.0 1.0 0.0 0 0 0 0)
  (Utilities|IsValid (Variables|Default|GetCubeInstance)
    (:Is%20Valid
      (Development|PrintString "Is Valid" false false)
      (CallFunction|DestroyCube (Variables|Default|GetCubeInstance)))
    (:Is%20Not%20Valid
      (Development|PrintString "Is Not Valid" false false)))
  (bind _returnvalue_2 (Game|SpawnActorfromClass "/Game/Blueprints/Mechaniques/Cube/BP_Cube.BP_Cube_C" (Math|Transform|MakeTransform (Math|Vector|MakeVector (.x (.location _returnvalue)) (.y (.location _returnvalue)) (- (.z (.location _returnvalue)) 1.4e+02)) "0, 0, 0" "1.000000,1.000000,1.000000") "Undefined" 0 0))
  (Variables|Default|SetCubeInstance _returnvalue_2))

(fn ConstructionScript)

(fn DestroyCube
  (params (CubeInstance :type Actor%20Object%20Reference))
  (Actor|DestroyActor CubeInstance))

(fn GetDeactivationTime
  (return 0.0))