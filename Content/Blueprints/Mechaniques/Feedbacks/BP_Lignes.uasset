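; BP_Lignes is a line feedback actor for mechanisms that shows an on/off state by switching its mesh between green and red materials.
; The construction script sets green when StartsActivated is true, red otherwise.
; Activate swaps to the opposite of that starting color and Deactivate restores it, so StartsActivated inverts the response.
; GetDeactivationTime always returns zero.
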(event EventBeginPlay)

(event Collision|EventActorBeginOverlap
  (params (OtherActor :type Actor%20Object%20Reference)))

(event EventTick
  (params (DeltaSeconds :type Float%20%28single-precision%29)))

(event EventActivate
  (if (Variables|Default|GetStartsActivated)
    (Rendering|Material|SetMaterial (Variables|Default|GetMesh) 0 "/Game/Levels/materials/M_Rouge.M_Rouge")
    (else
      (Rendering|Material|SetMaterial (Variables|Default|GetMesh) 0 "/Game/Levels/materials/M_Vert.M_Vert"))))

(event EventDeactivate
  (if (Variables|Default|GetStartsActivated)
    (Rendering|Material|SetMaterial (Variables|Default|GetMesh) 0 "/Game/Levels/materials/M_Vert.M_Vert")
    (else
      (Rendering|Material|SetMaterial (Variables|Default|GetMesh) 0 "/Game/Levels/materials/M_Rouge.M_Rouge"))))

(fn ConstructionScript
  (if (Variables|Default|GetStartsActivated)
    (Rendering|Material|SetMaterial (Variables|Default|GetMesh) 0 "/Game/Levels/materials/M_Vert.M_Vert")
    (else
      (Rendering|Material|SetMaterial (Variables|Default|GetMesh) 0 "/Game/Levels/materials/M_Rouge.M_Rouge"))))

(fn GetDeactivationTime
  (return 0.0))