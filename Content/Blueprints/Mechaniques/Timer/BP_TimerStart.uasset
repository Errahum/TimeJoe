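; BP_TimerStart is a trigger actor that starts the level timer when the first-person character overlaps it.
; On overlap it clears the character's scoreboard and timer animation-start flags and copies its Level value into the character's CurrentLevel.
; If the timer is not already on, it zeroes the character's minutes, seconds and deciseconds, turns the timer on and clears the finished-level flag.
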(event EventBeginPlay)

(event Collision|EventActorBeginOverlap
  (params (OtherActor :type Actor%20Object%20Reference))
  (bind _asbp_first_person_character (Utilities|Casting|CastToBP_FirstPersonCharacter OtherActor))
  (Variables|/Game/FirstPerson/Blueprints/BP_FirstPersonCharacter.BP_FirstPersonCharacter_C|SetScoreboardAnimationStart _asbp_first_person_character false)
  (Variables|/Game/FirstPerson/Blueprints/BP_FirstPersonCharacter.BP_FirstPersonCharacter_C|SetTimerAnimationStart _asbp_first_person_character false)
  (Variables|/Game/FirstPerson/Blueprints/BP_FirstPersonCharacter.BP_FirstPersonCharacter_C|SetCurrentLevel _asbp_first_person_character (Variables|Default|GetLevel))
  (if (not (Variables|/Game/FirstPerson/Blueprints/BP_FirstPersonCharacter.BP_FirstPersonCharacter_C|GetTimerOn _asbp_first_person_character))
    (Variables|/Game/FirstPerson/Blueprints/BP_FirstPersonCharacter.BP_FirstPersonCharacter_C|SetMinutes _asbp_first_person_character 0)
    (Variables|/Game/FirstPerson/Blueprints/BP_FirstPersonCharacter.BP_FirstPersonCharacter_C|SetSecondes _asbp_first_person_character 0)
    (Variables|/Game/FirstPerson/Blueprints/BP_FirstPersonCharacter.BP_FirstPersonCharacter_C|SetDeciSecondes _asbp_first_person_character 0)
    (Variables|/Game/FirstPerson/Blueprints/BP_FirstPersonCharacter.BP_FirstPersonCharacter_C|SetTimerOn _asbp_first_person_character true)
    (Variables|/Game/FirstPerson/Blueprints/BP_FirstPersonCharacter.BP_FirstPersonCharacter_C|SetFinishedLevel _asbp_first_person_character false)))

(event EventTick
  (params (DeltaSeconds :type Float%20%28single-precision%29)))

(fn ConstructionScript)