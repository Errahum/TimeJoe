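; BP_Piston_Mortel is a deadly piston that deals heavy damage to the first-person character on actor overlap.
; A timeline moves the piston along Z from its base height, triggered by Activate/Deactivate with delay and sound, or ping-ponging automatically when Looping.
; The construction script places the piston and sets the child laser FX length.
; GetDeactivationTime exposes a button deactivation time.
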(event Custom|Loop
  (Utilities|FlowControl|Delay (Variables|Delay|GetStartDelay))
  (bind _newtrack_0 (Timeline|Timeline Play)
    (:Update
      (Transformation|SetRelativeLocation (Variables|Default|GetPiston) (Math|Vector|MakeVector 0.0 0.0 (+ (* _newtrack_0 (Variables|Height|GetHeight)) (Variables|Height|GetBaseHeight))) false false))
    (:Finished
      (if (Variables|Default|GetLooping?)
        (Utilities|FlowControl|Delay (Variables|Delay|GetDelayInterval))
        (if (Variables|Default|GetReversing?)
          (Variables|Default|SetReversing? false)
          (Timeline|Timeline Play)
          (else
            (Variables|Default|SetReversing? true)
            (Timeline|Timeline Reverse)))))))

(event EventActivate
  (Utilities|FlowControl|Delay (Variables|Delay|GetStartDelay))
  (Audio|PlaySoundatLocation "/Game/Sounds/Piston/Prison_lift.Prison_lift" (Transformation|GetActorLocation) "0, 0, 0" 1.0 1.0 0.0 0 0 0 0)
  (bind _newtrack_0 (Timeline|Timeline Play)
    (:Update
      (Transformation|SetRelativeLocation (Variables|Default|GetPiston) (Math|Vector|MakeVector 0.0 0.0 (+ (* _newtrack_0 (Variables|Height|GetHeight)) (Variables|Height|GetBaseHeight))) false false))
    (:Finished
      (if (Variables|Default|GetLooping?)
        (Utilities|FlowControl|Delay (Variables|Delay|GetDelayInterval))
        (if (Variables|Default|GetReversing?)
          (Variables|Default|SetReversing? false)
          (Timeline|Timeline Play)
          (else
            (Variables|Default|SetReversing? true)
            (Timeline|Timeline Reverse)))))))

(event EventDeactivate
  (Utilities|FlowControl|Delay (Variables|Delay|GetStartDelay))
  (Audio|PlaySoundatLocation "/Game/Sounds/Piston/Prison_Reset.Prison_Reset" (Transformation|GetActorLocation) "0, 0, 0" 1.0 1.0 0.0 0 0 0 0)
  (bind _newtrack_0 (Timeline|Timeline Reverse)
    (:Update
      (Transformation|SetRelativeLocation (Variables|Default|GetPiston) (Math|Vector|MakeVector 0.0 0.0 (+ (* _newtrack_0 (Variables|Height|GetHeight)) (Variables|Height|GetBaseHeight))) false false))
    (:Finished
      (if (Variables|Default|GetLooping?)
        (Utilities|FlowControl|Delay (Variables|Delay|GetDelayInterval))
        (if (Variables|Default|GetReversing?)
          (Variables|Default|SetReversing? false)
          (Timeline|Timeline Play)
          (else
            (Variables|Default|SetReversing? true)
            (Timeline|Timeline Reverse)))))))

(event EventBeginPlay
  (if (Variables|Default|GetLooping?)
    (CallFunction|Loop)))

(event EventTick
  (params (DeltaSeconds :type Float%20%28single-precision%29))
  (Components|Timeline|SetPlayRate (Variables|Default|GetTimeline) (Variables|Default|GetPlayRate)))

(event Collision|EventActorBeginOverlap
  (params (OtherActor :type Actor%20Object%20Reference))
  (bind _asbp_first_person_character (Utilities|Casting|CastToBP_FirstPersonCharacter OtherActor))
  (Game|Damage|ApplyDamage _asbp_first_person_character 1e+02 0 0))

(fn ConstructionScript
  (Transformation|SetRelativeLocation (Variables|Default|GetPiston) (Math|Vector|MakeVector 0.0 0.0 (Variables|Height|GetBaseHeight)) false false)
  (bind _asbp_laser_fx (Utilities|Casting|CastToBP_LaserFX (Variables|/Script/Engine.ChildActorComponent|GetChildActor (Variables|Default|GetBP_LaserFX))))
  (Variables|/Game/Blueprints/Mechaniques/Laser/BP_LaserFX.BP_LaserFX_C|SetLongueur_Laser _asbp_laser_fx (Variables|Default|GetLongueur_Laser_Piston))
  (Transformation|SetRelativeScale3D (Variables|Default|GetBP_LaserFX) "1.000000,1.000000,1.000000"))

(fn GetDeactivationTime
  (return (Variables|Delay|GetBouton_Temps_Desactivation)))